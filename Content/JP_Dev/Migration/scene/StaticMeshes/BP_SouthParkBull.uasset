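; BP_SouthParkBull is an AI bull that wanders between random nearby reachable points, bobbing its mesh on a sine wave while grounded.
; Overlapping its BullMesh with a cube-carrying player raises its speed, never reset, and starts a charge.
; Touching a "Wall"-tagged actor stuns it briefly by disabling movement, then resumes wandering.
; Player overlap only tints the damage HUD; perception just stores a target, with focus logic left unconnected.
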(event `self.ReceiveBeginPlay`
  ; Bull AI wander
  (`self.MoveToRandomLocation`))

(event `MoveToRandomLocation`
  ; Bull AI wander
  (`|AIMoveTo` self (`NavigationSystemV1.K2_GetRandomReachablePointInRadius` (`self.K2_GetActorLocation`) 1000.0 null null) null
    (:`OnSuccess`
      (`KismetSystemLibrary.Delay` (`KismetMathLibrary.RandomFloatInRange` 0.5 2.5))
      (`self.MoveToRandomLocation`))))

(event `self.ReceiveTick`
  (params (DeltaSeconds :type "Float (single-precision)"))
  ; Hopping Code AI
  (if (`NavMovementComponent.IsMovingOnGround` (`self.CharacterMovement`))
    (`SceneComponent.K2_SetRelativeLocation` (`self.Mesh`) (`KismetMathLibrary.MakeVector` 0.0 0.0 (* (`KismetMathLibrary.Sin` (* (`KismetSystemLibrary.GetGameTimeInSeconds`) 25.0)) 20.0)) false false)))

(event `self.BullMesh.OnComponentBeginOverlap`
  (params (OverlappedComponent :type "PrimitiveComponent Object Reference") (OtherActor :type "Actor Object Reference") (OtherComp :type "PrimitiveComponent Object Reference") (OtherBodyIndex :type Integer) (bFromSweep :type Boolean) (SweepResult :type "HitResult Structure (by ref)"))
  ; AI Charge Player
  (bind _asbp_first_person_character_master (cast `/Game/_Developer/Sam/Blueprints/BP_FirstPersonCharacter_Master` OtherActor))
  (if (`/Game/_Developer/Sam/Blueprints/BP_FirstPersonCharacter_Master.bHasCube` _asbp_first_person_character_master)
    (bind _output_get (set `self.As BP First Person Character` _asbp_first_person_character_master))
    (set `CharacterMovementComponent.MaxWalkSpeed` 1000.0 (`self.CharacterMovement`))
    (`|AIMoveTo` self (0.0 0.0 0.0) _output_get)))

(event `self.NPCAI.OnTargetPerceptionUpdated`
  (params (Actor :type "Actor Object Reference") (Stimulus :type "AIStimulus Structure"))
  ; Targeting Perception
  (set `self.TargetActor` Actor))

(event `self.Capsule.OnComponentBeginOverlap`
  (params (OverlappedComponent :type "PrimitiveComponent Object Reference") (OtherActor :type "Actor Object Reference") (OtherComp :type "PrimitiveComponent Object Reference") (OtherBodyIndex :type Integer) (bFromSweep :type Boolean) (SweepResult :type "HitResult Structure (by ref)"))
  ; Stunned
  (if (`self.ActorHasTag` OtherActor "Wall")
    (`Controller.StopMovement` (`AIBlueprintHelperLibrary.GetAIController` self))
    (`CharacterMovementComponent.SetMovementMode` (`self.CharacterMovement`) "MOVE_None" 0)
    (`KismetSystemLibrary.Delay` 2.0)
    (`CharacterMovementComponent.SetMovementMode` (`self.CharacterMovement`) "MOVE_NavWalking" 0)
    (`self.MoveToRandomLocation`)))

(event `self.ReceiveActorBeginOverlap`
  (params (OtherActor :type "Actor Object Reference"))
  ; Health & Damage Code
  (bind _asbp_first_person_character_master (cast `/Game/_Developer/Sam/Blueprints/BP_FirstPersonCharacter_Master` OtherActor))
  (`UserWidget.SetColorAndOpacity` (`/Game/Emma_Dev/Widgets/WBP_BullMiniGame.WBP_Damage` (`/Game/_Developer/Sam/Blueprints/BP_FirstPersonCharacter_Master.BullHud` _asbp_first_person_character_master)) (make `LinearColor` 1.0 0.0 0.0 1.0)))

(event `self.ReceiveActorEndOverlap`
  (params (OtherActor :type "Actor Object Reference"))
  ; Health & Damage Code
  (bind _asbp_first_person_character_master (cast `/Game/_Developer/Sam/Blueprints/BP_FirstPersonCharacter_Master` OtherActor))
  (`UserWidget.SetColorAndOpacity` (`/Game/Emma_Dev/Widgets/WBP_BullMiniGame.WBP_Damage` (`/Game/_Developer/Sam/Blueprints/BP_FirstPersonCharacter_Master.BullHud` _asbp_first_person_character_master)) (make `LinearColor` 0.0)))

(fn `UserConstructionScript`)