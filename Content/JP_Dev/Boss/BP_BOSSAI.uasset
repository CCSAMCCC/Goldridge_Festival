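; BP_BOSSAI is the boss character, feeding combat events into its AI controller's blackboard.
; PawnSensing flags chase range when it sees the first-person player.
; Damage events decrement a hit counter; each depletion sets metHitCount, resets it and spends a flee count, destroying the boss at zero.
; SetStun zeroes walk speed; its hardcoded true condition leaves the speed-restore branch unreachable.
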(event `Set Stun`
  (if true
    (set `CharacterMovementComponent.MaxWalkSpeed` 0.0 (`self.CharacterMovement`))
    (else
      (set `CharacterMovementComponent.MaxWalkSpeed` 200.0 (`self.CharacterMovement`)))))

(event `self.PawnSensing.OnSeePawn`
  (params (Pawn :type "Pawn Object Reference"))
  (cast `/Game/_Developer/Sam/Blueprints/BP_FirstPersonCharacter_Master` Pawn)
  (`BlackboardComponent.SetValueAsBool` (`AIBlueprintHelperLibrary.GetBlackboard` (`AIBlueprintHelperLibrary.GetAIController` self)) "isInChaseRange?" true))

(event `LowerHealth`
  (set `self.HitCount` (- (`self.HitCount`) 1) :!label _label)
  (if (<= (`self.HitCount`) 0)
    (set `self.FleeCount` (- (`self.FleeCount`) 1))
    (`BlackboardComponent.SetValueAsBool` (`AIBlueprintHelperLibrary.GetBlackboard` (`AIBlueprintHelperLibrary.GetAIController` self)) "metHitCount" true)
    (set `self.HitCount` 3)
    (if (== (`self.FleeCount`) 0)
      (`self.K2_DestroyActor`))))

(event `/Game/Shaon/BPI_Damage.SendDamage`
  (params (Damage :type Integer))
  (`KismetSystemLibrary.PrintString` "Boss Got Damaged")
  (goto _label))

(fn `UserConstructionScript`)