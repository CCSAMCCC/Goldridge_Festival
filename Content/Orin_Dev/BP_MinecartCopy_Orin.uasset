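; Player-driven minecart character for a track-riding minigame with dynamite throwing, points and a leaderboard.
; Tick moves the capsule along the current track spline using MaxWalkSpeed as speed, boosted downhill; SwitchTracks jumps to the next spline.
; Enhanced Input drives acceleration, braking, ducking and timeline-animated leaning, where over-holding a lean triggers game over.
; Throwing attaches dynamite to the hand, then launches it on a suggested arc, aimed at overlapped gold ore, unless stunned.
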(event `self.ReceiveBeginPlay`
  (`self.Setup Inputs`)
  (bind _outactors (`GameplayStatics.GetAllActorsOfClassWithTag` "/Game/Orin_Dev/BP_StraightTrack.BP_StraightTrack_C" "StartPoint"))
  (set `self.CurrentSplineRef` (`|GetArrayItem` _outactors))
  (bind _returnvalue (`|CreateWidget` "/Game/Shaon/Widgets/W_Leaderboard.W_Leaderboard_C"))
  (set `self.Leaderboard` _returnvalue)
  (set `self.bIsSwitching` false)
  (set `self.bLeaningLeft` false)
  (set `self.bLeaningRight` false))

(event `self.ReceiveTick`
  (params (DeltaSeconds :type "Float (single-precision)"))
  ; Movement along a spline
  (if (`self.bCanMove`)
    (bind _output_get (set `self.SplineDistance` (+ (* DeltaSeconds (`CharacterMovementComponent.MaxWalkSpeed` (`self.CharacterMovement`))) (`self.SplineDistance`))))
    (bind _returnvalue (`SplineComponent.GetTransformAtDistanceAlongSpline` (`/Game/Orin_Dev/BP_StraightTrack.Spline` (`self.CurrentSplineRef`)) _output_get "World" false))
    (`SceneComponent.K2_SetRelativeTransform` (`self.CapsuleComponent`) (`KismetMathLibrary.MakeTransform` (`KismetMathLibrary.MakeVector` (- (.x (.location _returnvalue)) 10.0) (.y (.location _returnvalue)) (+ (.z (.location _returnvalue)) 95.0)) (.rotation _returnvalue) (`SceneComponent.RelativeScale3D` (`self.CapsuleComponent`))) false false)
    (if (< (.pitch (.rotation (`SplineComponent.GetTransformAtDistanceAlongSpline` (`/Game/Orin_Dev/BP_StraightTrack.Spline` (`self.CurrentSplineRef`)) (`self.SplineDistance`) "World" false))) -5.0)
      (if (`self.bCanSpeedUp`)
        (set `self.bCanSpeedUp` false)
        (set `CharacterMovementComponent.MaxWalkSpeed` (+ (`self.CurrentSpeed`) 500.0) (`self.CharacterMovement`)))
      (else
        (set `CharacterMovementComponent.MaxWalkSpeed` (`self.CurrentSpeed`) (`self.CharacterMovement`))
        (set `self.bCanSpeedUp` true)))))

(event `EnhancedInput|/Game/Kaitlyn_Dev/IA_MinecartGo`
  (params (ActionValue :type "Float (double-precision)") (ElapsedSeconds :type "Float (double-precision)") (TriggeredSeconds :type "Float (double-precision)") (InputAction :type "InputAction Object Reference" :default "/Game/Kaitlyn_Dev/IA_MinecartGo.IA_MinecartGo"))
  (bind _charactermovement (`self.CharacterMovement`))
  (bind (_relativerotation_roll _relativerotation_pitch _relativerotation_yaw) (`KismetMathLibrary.BreakRotator` (`SceneComponent.RelativeRotation` (`self.Minecart`))))
  ; Forward movement with acceleration for minecart
  (:`Triggered`
    (if (not (`self.bCanMove`))
      (set `self.bCanMove` true))
    (`self.AddMovementInput` (`KismetMathLibrary.GetForwardVector` (`self.GetControlRotation`)) ActionValue)
    (bind (_direction _newtrack_0) (`Timeline|ForwardRotationTimeline` :!label _label)
      (:`Update`
        (`SceneComponent.K2_SetRelativeRotation` (`self.Minecart`) (`KismetMathLibrary.MakeRotator` _newtrack_0 _relativerotation_pitch _relativerotation_yaw) false false)
        (bind _output_get (set `CharacterMovementComponent.MaxWalkSpeed` (`KismetMathLibrary.FClamp` (+ (`CharacterMovementComponent.MaxWalkSpeed` _charactermovement) (`self.SpeedIncrease`)) 200.0 (`self.MaxSpeed`)) _charactermovement :!label _label_2))
        (set `self.CurrentSpeed` _output_get)
        (`KismetSystemLibrary.Delay` 5.0)
        (goto _label_2))))
  (:`Completed`
    (bind _output_get_2 (set `CharacterMovementComponent.MaxWalkSpeed` (`self.NormalSpeed`) (`self.CharacterMovement`)))
    (set `self.CurrentSpeed` _output_get_2)
    (goto _label :!via `Reverse`)))

(event `SwitchTracks`
  ; Code to switch the minecart over to another spline
  (if (not (`self.bIsSwitching`))
    (set `self.bIsSwitching` true)
    (bind _output_get (set `self.SplineDistance` 0.0))
    (bind _returnvalue (`SplineComponent.GetTransformAtDistanceAlongSpline` (`/Game/Orin_Dev/BP_StraightTrack.Spline` (`self.NextSplineRef`)) _output_get "World" false))
    (`SceneComponent.K2_SetRelativeTransform` (`self.CapsuleComponent`) (`KismetMathLibrary.MakeTransform` (`KismetMathLibrary.MakeVector` (.x (.location _returnvalue)) (.y (.location _returnvalue)) (+ (.z (.location _returnvalue)) 100.0)) (.rotation _returnvalue) (`SceneComponent.RelativeScale3D` (`self.CapsuleComponent`))) false false)
    (set `self.CurrentSplineRef` (`self.NextSplineRef`))
    (set `self.bCanMove` true)
    (set `self.bIsSwitching` false)))

(event `EnhancedInput|/Game/Kaitlyn_Dev/IA_MinecartBrake`
  (params (ActionValue :type "Float (double-precision)") (ElapsedSeconds :type "Float (double-precision)") (TriggeredSeconds :type "Float (double-precision)") (InputAction :type "InputAction Object Reference" :default "/Game/Kaitlyn_Dev/IA_MinecartBrake.IA_MinecartBrake"))
  (bind _charactermovement (`self.CharacterMovement`))
  (bind (_relativerotation_roll _relativerotation_pitch _relativerotation_yaw) (`KismetMathLibrary.BreakRotator` (`SceneComponent.RelativeRotation` (`self.Minecart`))))
  ; Braking for Minecart
  (:`Triggered`
    (bind (_direction _newtrack_0) (`Timeline|BrakeRotationTimeline` :!label _label_3)
      (:`Update`
        (`SceneComponent.K2_SetRelativeRotation` (`self.Minecart`) (`KismetMathLibrary.MakeRotator` _newtrack_0 _relativerotation_pitch _relativerotation_yaw) false false)
        (bind _output_get (set `CharacterMovementComponent.MaxWalkSpeed` (`KismetMathLibrary.FClamp` (- (`CharacterMovementComponent.MaxWalkSpeed` _charactermovement) (`self.BrakingAmount`)) 200.0 (`self.MaxSpeed`)) _charactermovement :!label _label_4))
        (set `self.CurrentSpeed` _output_get)
        (`KismetSystemLibrary.Delay` 5.0)
        (goto _label_4))))
  (:`Completed`
    (bind _output_get_2 (set `CharacterMovementComponent.MaxWalkSpeed` (`self.NormalSpeed`) (`self.CharacterMovement`)))
    (set `self.CurrentSpeed` _output_get_2)
    (goto _label_3 :!via `Reverse`)))

(event `EnhancedInput|/Game/Kaitlyn_Dev/IA_MinecartLeftLean`
  (params (ActionValue :type Boolean) (ElapsedSeconds :type "Float (double-precision)") (TriggeredSeconds :type "Float (double-precision)") (InputAction :type "InputAction Object Reference" :default "/Game/Kaitlyn_Dev/IA_MinecartLeftLean.IA_MinecartLeftLean"))
  (bind _minecart (`self.Minecart`))
  (bind (_relativerotation_roll _relativerotation_pitch _relativerotation_yaw) (`KismetMathLibrary.BreakRotator` (`SceneComponent.RelativeRotation` _minecart)))
  ; Leaning for Minecart
  (:`Triggered`
    (if (not (`self.bLeaningRight`))
      (set `self.bLeaningLeft` true)
      (if (`KismetMathLibrary.NearlyEqual_FloatFloat` (.pitch (.rotation (`SceneComponent.GetRelativeTransform` (`self.Minecart`)))) 0.0 1.0)
        (bind (_direction _newtrack_0) (`Timeline|LeftLeanTimeline` :!label _label_5)
          (:`Update`
            (`SceneComponent.K2_SetRelativeRotation` _minecart (`KismetMathLibrary.MakeRotator` _relativerotation_roll _newtrack_0 _relativerotation_yaw) false false)
            (if (> TriggeredSeconds 5.0)
              (`self.GameOver`)))))))
  (:`Completed`
    (set `self.bLeaningLeft` false)
    (goto _label_5 :!via `Reverse`)))

(event `EnhancedInput|/Game/Kaitlyn_Dev/IA_MinecartRightLean`
  (params (ActionValue :type Boolean) (ElapsedSeconds :type "Float (double-precision)") (TriggeredSeconds :type "Float (double-precision)") (InputAction :type "InputAction Object Reference" :default "/Game/Kaitlyn_Dev/IA_MinecartRightLean.IA_MinecartRightLean"))
  (bind _minecart (`self.Minecart`))
  (bind (_relativerotation_roll _relativerotation_pitch _relativerotation_yaw) (`KismetMathLibrary.BreakRotator` (`SceneComponent.RelativeRotation` _minecart)))
  ; Leaning for Minecart
  (:`Triggered`
    (if (not (`self.bLeaningLeft`))
      (set `self.bLeaningRight` true)
      (if (`KismetMathLibrary.NearlyEqual_FloatFloat` (.pitch (.rotation (`SceneComponent.GetRelativeTransform` (`self.Minecart`)))) 0.0 1.0)
        (bind (_direction _newtrack_0) (`Timeline|LeanRightTimeline` :!label _label_6)
          (:`Update`
            (`SceneComponent.K2_SetRelativeRotation` _minecart (`KismetMathLibrary.MakeRotator` _relativerotation_roll _newtrack_0 _relativerotation_yaw) false false)
            (if (> TriggeredSeconds 5.0)
              (`self.GameOver`)))))))
  (:`Completed`
    (set `self.bLeaningRight` false)
    (goto _label_6 :!via `Reverse`)))

(event `EnhancedInput|/Game/Kaitlyn_Dev/IA_MinecartDuck`
  (params (ActionValue :type Boolean) (ElapsedSeconds :type "Float (double-precision)") (TriggeredSeconds :type "Float (double-precision)") (InputAction :type "InputAction Object Reference" :default "/Game/Kaitlyn_Dev/IA_MinecartDuck.IA_MinecartDuck"))
  (bind _capsulecomponent (`self.CapsuleComponent`))
  (bind _capsulecomponent_2 (`self.CapsuleComponent`))
  (bind (_relativelocation_x _relativelocation_y _relativelocation_z) (`KismetMathLibrary.BreakVector` (`SceneComponent.RelativeLocation` _capsulecomponent_2)))
  (bind (_relativelocation_x_2 _relativelocation_y_2 _relativelocation_z_2) (`KismetMathLibrary.BreakVector` (`SceneComponent.RelativeLocation` _capsulecomponent)))
  ; Ducking while in the minecart
  (:`Started`
    (`SceneComponent.K2_SetRelativeLocation` _capsulecomponent (`KismetMathLibrary.MakeVector` _relativelocation_x_2 _relativelocation_y_2 (- _relativelocation_z_2 40.0)) false false)
    (`KismetSystemLibrary.PrintString` "I'm ducking"))
  (:`Completed`
    (`SceneComponent.K2_SetRelativeLocation` _capsulecomponent_2 (`KismetMathLibrary.MakeVector` _relativelocation_x _relativelocation_y (+ _relativelocation_z 40.0)) false false)
    (`KismetSystemLibrary.PrintString` "Returned to normal")))

(event `Key|G`
  (params (Key :type "Key Structure"))
  ; Exiting the minecart
  (:`Pressed`
    (`KismetSystemLibrary.PrintString` "Exiting minecart")
    (`GameplayStatics.OpenLevelBySoftObjectPtr` "/Game/Kaitlyn_Dev/Lvl_1stPersonTesting.Lvl_1stPersonTesting") ; Change this to level you you want to return to
  ))

(event `GameOver`
  (`self.DisableInput` null)
  (`KismetSystemLibrary.PrintString` "Game Over!"))

(event `EnhancedInput|/Game/Kaitlyn_Dev/IA_Throw`
  (params (ActionValue :type Boolean) (ElapsedSeconds :type "Float (double-precision)") (TriggeredSeconds :type "Float (double-precision)") (InputAction :type "InputAction Object Reference" :default "/Game/Kaitlyn_Dev/IA_Throw.IA_Throw"))
  (bind _dynamiteref (`self.DynamiteRef`))
  (bind _dynamiteref_2 (`self.DynamiteRef`))
  (bind _stunned (`self.Stunned`))
  ; Throwing for Minecart
  (:`Triggered`
    (if (not _stunned)
      (bind _dynamiteref_3 (`self.DynamiteRef`)
        (:`then`
          (`self.K2_DetachFromActor` _dynamiteref_3 "KeepWorld" "KeepWorld" "KeepWorld")
          (`ActorComponent.Activate` (`/Game/Kaitlyn_Dev/BP_Dynamite.ProjectileMovement` _dynamiteref_3) false)
          (`KismetSystemLibrary.Delay` 0.5)
          (`PrimitiveComponent.SetCollisionEnabled` (`/Game/Kaitlyn_Dev/BP_Dynamite.Cylinder` (`self.DynamiteRef`)) "QueryAndPhysics")
          (`PrimitiveComponent.SetSimulatePhysics` (`/Game/Kaitlyn_Dev/BP_Dynamite.Cylinder` (`self.DynamiteRef`)) true)
          (`PrimitiveComponent.AddVelocityChangeImpulseAtLocation` (`/Game/Kaitlyn_Dev/BP_Dynamite.Cylinder` (`self.DynamiteRef`)) (`MovementComponent.Velocity` (`/Game/Kaitlyn_Dev/BP_Dynamite.ProjectileMovement` (`self.DynamiteRef`))) (`SceneComponent.K2_GetComponentLocation` (`/Game/Kaitlyn_Dev/BP_Dynamite.Cylinder` (`self.DynamiteRef`))) "None")
          (set `self.bCanThrow` true)
          (`KismetSystemLibrary.Delay` 1.5)
          (`self.K2_DestroyActor` (`self.DynamiteRef`)))
        (:`else`))))
  (:`Started`
    (if _stunned
      _
      (elif (`self.bCanThrow`)
        (set `self.bCanThrow` false)
        (bind _returnvalue (`|SpawnActorFromClass` "/Game/Kaitlyn_Dev/BP_Dynamite.BP_Dynamite_C" (`self.GetTransform`) "Undefined" "MultiplyWithRoot" null null null null))
        (set `self.DynamiteRef` _returnvalue)
        (`PrimitiveComponent.SetCollisionEnabled` (`/Game/Kaitlyn_Dev/BP_Dynamite.Cylinder` _returnvalue) "NoCollision")
        (`self.K2_AttachToComponent` (`self.DynamiteRef`) (`self.PlayerVisual`) "HandGrip_R" "SnapToTarget" "SnapToTarget" "SnapToTarget" true)
        (if (`self.bOverlappedGoldOre`)
          (bind (_outlaunchvelocity _returnvalue_2) (`GameplayStatics.SuggestProjectileVelocity_CustomArc` (`SceneComponent.K2_GetComponentLocation` (`/Game/Kaitlyn_Dev/BP_Dynamite.Cylinder` (`self.DynamiteRef`))) (`self.OreLocation`)))
          (if _returnvalue_2
            (bind _output_get (set `MovementComponent.Velocity` _outlaunchvelocity (`/Game/Kaitlyn_Dev/BP_Dynamite.ProjectileMovement` _dynamiteref)))
            (`GameplayStatics.Blueprint_PredictProjectilePath_Advanced` (make `PredictProjectilePathParams` (`SceneComponent.K2_GetComponentLocation` (`/Game/Kaitlyn_Dev/BP_Dynamite.Cylinder` _dynamiteref)) _output_get true 0.0 5.0 true "ECC_Visibility")))
          (else
            (`KismetSystemLibrary.PrintString` "No overlapped Gold")
            (bind (_outlaunchvelocity_2 _returnvalue_3) (`GameplayStatics.SuggestProjectileVelocity_CustomArc` (`SceneComponent.K2_GetComponentLocation` (`/Game/Kaitlyn_Dev/BP_Dynamite.Cylinder` (`self.DynamiteRef`))) (`SceneComponent.GetForwardVector` (`self.Minecart`))))
            (if _returnvalue_3
              (bind _output_get_2 (set `MovementComponent.Velocity` _outlaunchvelocity_2 (`/Game/Kaitlyn_Dev/BP_Dynamite.ProjectileMovement` _dynamiteref_2)))
              (`GameplayStatics.Blueprint_PredictProjectilePath_Advanced` (make `PredictProjectilePathParams` (`SceneComponent.K2_GetComponentLocation` (`/Game/Kaitlyn_Dev/BP_Dynamite.Cylinder` _dynamiteref_2)) _output_get_2 true 0.0 5.0 true "ECC_Visibility")))))
        (else
          (`KismetSystemLibrary.PrintString` "Must wait before throwing agian" true true (struct :`R` 0.116767 :`G` 1.0 :`B` 0.126042 :`A` 1.0)))))))

(event `CustomEvent`
  (params (Points :type Integer))
  ;[1 0.9545 0 0.5] Points
  (set `self.Points` (+ (`self.Points`) Points)))

(event `UpdateLeaderboardDisplay`
  (params (Scoreboard :type "Array of Integer") (Names :type "Array of String"))
  ;[0.03632 0.15 0.01788 0.5] Leaderboard
  (set `self.Scoreboard` Scoreboard)
  (set `self.Names` Names)
  (for (_array_element _array_index) (`/Game/Shaon/Widgets/W_Leaderboard.Scoreboard` (`self.Leaderboard`))
    (set `TextBlock.Text` (`KismetTextLibrary.Conv_StringToText` (`KismetStringLibrary.Concat_StrStr` (`KismetStringLibrary.Conv_IntToString` (- 10 _array_index)) ".    " (`|GetArrayItem` (`self.Names`) _array_index) "   " (`KismetStringLibrary.Conv_IntToString` (`|GetArrayItem` (`self.Scoreboard`) _array_index)) " pts")) _array_element)))

(event `Display leaderboard`
  ;[0.03632 0.15 0.01788 0.5] Leaderboard
  (`UserWidget.AddToViewport` (`self.Leaderboard`) 0)
  (`KismetSystemLibrary.Delay` 5.0)
  (`Widget.RemoveFromParent` (`self.Leaderboard`)))

(event `EnterStunDelay`
  (set `self.Stunned` true)
  (`KismetSystemLibrary.Delay` (`self.StunDuration`))
  (set `self.Stunned` false))

(fn `GetPoints`
  (returns (GetPoints :type Integer))
  (return 0))

(fn `Interact`
  (params (Interactor :type "Character Object Reference"))
  (returns (Success :type Boolean))
  (`KismetSystemLibrary.PrintString` "Getting into Minecart!")
  (`GameplayStatics.OpenLevelBySoftObjectPtr` "/Game/Kaitlyn_Dev/Lvl_MinecartTests.Lvl_MinecartTests")
  (return false))

(fn `Setup Inputs`
  (`EnhancedInputSubsystemInterface.AddMappingContext` (pcsubsystem `EnhancedInputLocalPlayerSubsystem` (`GameplayStatics.GetPlayerController` 0)) "/Game/Kaitlyn_Dev/IMC_Minecart.IMC_Minecart" 0 (struct)))

(fn `UserConstructionScript`)