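; Straight rail track that builds its mesh along a spline and lets a leaning minecart switch onto it.
; The construction script lays spline mesh segments at mesh-length intervals, with clamped tangents.
; On box overlap, a non-switching BP_MinecartCopy_Orin leaning toward the track's Right or Left tag takes this actor as next spline and calls SwitchTracks.
; The end-overlap reset of IsSwitching is disconnected and never runs.
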(event `self.Box.OnComponentBeginOverlap`
  (params (OverlappedComponent :type "PrimitiveComponent Object Reference") (OtherActor :type "Actor Object Reference") (OtherComp :type "PrimitiveComponent Object Reference") (OtherBodyIndex :type Integer) (bFromSweep :type Boolean) (SweepResult :type "HitResult Structure (by ref)"))
  ; Checks the tag of the rail, compares it to the current lean state of the minecart and assigns new spline accordingly
  (bind _asbp_minecart_copy_orin (cast `/Game/Orin_Dev/BP_MinecartCopy_Orin` OtherActor))
  (if (`/Game/Orin_Dev/BP_MinecartCopy_Orin.bIsSwitching` _asbp_minecart_copy_orin)
    _
    (elif (`self.ActorHasTag` "Right")
      (if (`/Game/Orin_Dev/BP_MinecartCopy_Orin.bLeaningRight` _asbp_minecart_copy_orin)
        (set `/Game/Orin_Dev/BP_MinecartCopy_Orin.NextSplineRef` self _asbp_minecart_copy_orin)
        (`/Game/Orin_Dev/BP_MinecartCopy_Orin.SwitchTracks` _asbp_minecart_copy_orin))
      (elif (`self.ActorHasTag` "Left")
        (if (`/Game/Orin_Dev/BP_MinecartCopy_Orin.bLeaningLeft` _asbp_minecart_copy_orin)
          (set `/Game/Orin_Dev/BP_MinecartCopy_Orin.NextSplineRef` self _asbp_minecart_copy_orin)
          (`/Game/Orin_Dev/BP_MinecartCopy_Orin.SwitchTracks` _asbp_minecart_copy_orin))))))

(event `self.ReceiveActorEndOverlap`
  (params (OtherActor :type "Actor Object Reference"))
  ; Allows the minecart to swap again AFTER its swap to prevent infinite loop
  (bind _asbp_minecart_copy_orin (cast `/Game/Orin_Dev/BP_MinecartCopy_Orin` OtherActor)))

(fn `UserConstructionScript`
  (bind _spline (`self.Spline`))
  (bind _spline_2 (`self.Spline`))
  (bind (_min _max) (break `Box` (`StaticMesh.GetBoundingBox` (`self.SplineMesh`))))
  (set `self.MeshLength` (.x (- _max _min)))
  (for _index (range (+ (`KismetMathLibrary.FTrunc` (/ (`SplineComponent.GetSplineLength` (`self.Spline`)) (`self.MeshLength`))) 1))
    ; Spawns the mesh and sets the direction
    (bind _returnvalue (`AddComponent|NODE_AddSplineMeshComponent-0`))
    (`StaticMeshComponent.SetStaticMesh` _returnvalue (`self.SplineMesh`))
    (`SplineMeshComponent.SetForwardAxis` _returnvalue "X" true)
    (bind _returnvalue_2 (* _index (`self.MeshLength`)))
    (bind _returnvalue_3 (* (+ _index 1) (`self.MeshLength`)))
    (`SplineMeshComponent.SetStartAndEnd` _returnvalue (`SplineComponent.GetLocationAtDistanceAlongSpline` _spline _returnvalue_2 "Local") (`KismetMathLibrary.ClampVectorSize` (`SplineComponent.GetTangentAtDistanceAlongSpline` _spline _returnvalue_2 "Local") 0.0 (`self.MeshLength`)) (`SplineComponent.GetLocationAtDistanceAlongSpline` _spline_2 _returnvalue_3 "Local") (`KismetMathLibrary.ClampVectorSize` (`SplineComponent.GetTangentAtDistanceAlongSpline` _spline_2 _returnvalue_3 "Local") 0.0 (`self.MeshLength`)) true)))