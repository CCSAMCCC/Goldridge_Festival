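; Spline-based minecart rail that builds its track from repeated spline meshes in the construction script and handles track switching.
; Actor tags set behavior: on box overlap, Jump rails switch the cart once automatically, while Left or Right rails require a matching lean.
; Broken Left or Right rails also become active and tint a lean widget red.
; While active, Tick calls the cart's GameOver if that lean is lost.
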(event `self.ReceiveTick`
  (params (DeltaSeconds :type "Float (single-precision)"))
  ;[0 0.9379 1 0.5] Rail Swicthing checks based on the tags applied to the rail itself
  ;;[1 0 0.000559 0.5] If in the active state from a broken rail, checks to see if the player is leaning correctly
  (if (`self.isActive`)
    (if (`self.ActorHasTag` "Right")
      (if (not (`/Game/Kaitlyn_Dev/BP_Minecart_Kaitlyn.bLeaningRight` (stale `self.Box.OnComponentBeginOverlap` _asbp_minecart_kaitlyn)))
        (`/Game/Kaitlyn_Dev/BP_Minecart_Kaitlyn.GameOver` (stale `self.Box.OnComponentBeginOverlap` _asbp_minecart_kaitlyn)))
      (elif (`self.ActorHasTag` "Left")
        (if (not (`/Game/Kaitlyn_Dev/BP_Minecart_Kaitlyn.bLeaningLeft` (stale `self.Box.OnComponentBeginOverlap` _asbp_minecart_kaitlyn)))
          (`/Game/Kaitlyn_Dev/BP_Minecart_Kaitlyn.GameOver` (stale `self.Box.OnComponentBeginOverlap` _asbp_minecart_kaitlyn)))))))

(event `self.Box.OnComponentBeginOverlap`
  (params (OverlappedComponent :type "PrimitiveComponent Object Reference") (OtherActor :type "Actor Object Reference") (OtherComp :type "PrimitiveComponent Object Reference") (OtherBodyIndex :type Integer) (bFromSweep :type Boolean) (SweepResult :type "HitResult Structure (by ref)"))
  ;[0 0.9379 1 0.5] Rail Swicthing checks based on the tags applied to the rail itself
  (bind _asbp_minecart_kaitlyn (cast `/Game/Kaitlyn_Dev/BP_Minecart_Kaitlyn` OtherActor))
  (if (`/Game/Kaitlyn_Dev/BP_Minecart_Kaitlyn.bIsSwitching` _asbp_minecart_kaitlyn)
    _
    (elif (`self.ActorHasTag` "Jump")
      (`/Engine/EditorBlueprintResources/StandardMacros.DoOnce` false
        (:`Completed`
          (set `/Game/Kaitlyn_Dev/BP_Minecart_Kaitlyn.NextSplineRef` self _asbp_minecart_kaitlyn)
          (`/Game/Kaitlyn_Dev/BP_Minecart_Kaitlyn.SwitchTracks` _asbp_minecart_kaitlyn)))
      (elif (`self.ActorHasTag` "Right")
        (if (`/Game/Kaitlyn_Dev/BP_Minecart_Kaitlyn.bLeaningRight` _asbp_minecart_kaitlyn)
          (`/Engine/EditorBlueprintResources/StandardMacros.DoOnce` false
            (:`Completed`
              (set `/Game/Kaitlyn_Dev/BP_Minecart_Kaitlyn.NextSplineRef` self _asbp_minecart_kaitlyn)
              (if (`self.ActorHasTag` "Broken")
                (set `self.isActive` true)
                (bind _minecarwidget (`/Game/Kaitlyn_Dev/BP_Minecart_Kaitlyn.MinecarWidget` _asbp_minecart_kaitlyn))
                (`UserWidget.SetColorAndOpacity` (`/Game/Emma_Dev/Widgets/WBP_MinecartMinigame.WBP_LeanLeft` _minecarwidget) (make `LinearColor` 1.0 0.0 0.0 1.0)))
              (`/Game/Kaitlyn_Dev/BP_Minecart_Kaitlyn.SwitchTracks` _asbp_minecart_kaitlyn))))
        (elif (`self.ActorHasTag` "Left")
          (if (`/Game/Kaitlyn_Dev/BP_Minecart_Kaitlyn.bLeaningLeft` _asbp_minecart_kaitlyn)
            (`/Engine/EditorBlueprintResources/StandardMacros.DoOnce` false
              (:`Completed`
                (set `/Game/Kaitlyn_Dev/BP_Minecart_Kaitlyn.NextSplineRef` self _asbp_minecart_kaitlyn)
                (if (`self.ActorHasTag` "Broken")
                  (set `self.isActive` true)
                  (`UserWidget.SetColorAndOpacity` (`/Game/Emma_Dev/Widgets/WBP_MinecartMinigame.WBP_LeanRight` _minecarwidget) (make `LinearColor` 1.0 0.0 0.0 1.0)))
                (`/Game/Kaitlyn_Dev/BP_Minecart_Kaitlyn.SwitchTracks` _asbp_minecart_kaitlyn)))))))))

(fn `UserConstructionScript`
  (bind _spline (`self.Spline`))
  (bind _spline_2 (`self.Spline`))
  (bind (_min _max) (break `Box` (`StaticMesh.GetBoundingBox` (`self.SplineMesh`))))
  (set `self.MeshLength` (.x (- _max _min)))
  (for _index (range (+ (`KismetMathLibrary.FTrunc` (/ (`SplineComponent.GetSplineLength` (`self.Spline`)) (`self.MeshLength`))) 1))
    ; Spawns the mesh and sets the direction
    (bind _returnvalue (`AddComponent|NODE_AddSplineMeshComponent-0`))
    (`StaticMeshComponent.SetStaticMesh` _returnvalue (`self.SplineMesh`))
    (`SplineMeshComponent.SetForwardAxis` _returnvalue "X" true)
    (bind _returnvalue_2 (* _index (`self.MeshLength`)))
    (bind _returnvalue_3 (* (+ _index 1) (`self.MeshLength`)))
    (`SplineMeshComponent.SetStartAndEnd` _returnvalue (`SplineComponent.GetLocationAtDistanceAlongSpline` _spline _returnvalue_2 "Local") (`KismetMathLibrary.ClampVectorSize` (`SplineComponent.GetTangentAtDistanceAlongSpline` _spline _returnvalue_2 "Local") 0.0 (`self.MeshLength`)) (`SplineComponent.GetLocationAtDistanceAlongSpline` _spline_2 _returnvalue_3 "Local") (`KismetMathLibrary.ClampVectorSize` (`SplineComponent.GetTangentAtDistanceAlongSpline` _spline_2 _returnvalue_3 "Local") 0.0 (`self.MeshLength`)) true)))