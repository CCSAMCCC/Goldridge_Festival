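; Player character for the minecart minigame, riding BP_TestingRail_Orin splines with throttle, brake, duck, lean and dynamite throwing.
; Tick advances spline distance from walk speed, a multiplier and cart tilt; SwitchTracks jumps to the next spline, while looping timers drive leaning.
; Throws target the nearest in-range ore with a predicted arc, and repeated mistimed throws cause a stun slowdown.
; Also handles points, HUD, leaderboard, pause menu and a physics-launched game over.
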(event Custom|UpdateLeaderboardDisplay
  (params (Scoreboard :type Array%20of%20Integers) (Names :type Array%20of%20Strings))
  ;[0.03632 0.15 0.01788 0.5] Leaderboard
  (Variables|Score|SetScoreboard Scoreboard)
  (Variables|Score|SetNames Names)
  (for (_array_element _array_index) (Variables|/Game/Shaon/Widgets/W_Leaderboard.W_Leaderboard_C|GetScoreboard (Variables|Score|GetLeaderboard))
    (Variables|/Script/UMG.TextBlock|SetText _array_element (Utilities|Text|ToText(String) (Utilities|String|Append (Utilities|String|ToString(Integer) (- 10 _array_index)) ".    " (Utilities|Array|Get(acopy) (Variables|Score|GetNames) _array_index) "   " (Utilities|String|ToString(Integer) (Utilities|Array|Get(acopy) (Variables|Score|GetScoreboard) _array_index)) " pts")))))

(event Custom|GameOver
  (bind _minecart (Variables|Default|GetMinecart))
  (bind _relativerotation (Variables|/Script/Engine.SceneComponent|GetRelativeRotation _minecart))
  (bind _returnvalue (< (.pitch _relativerotation) 0.0))
  (bind _returnvalue_2 (Math|Float|SelectFloat -1.0 1.0 _returnvalue))
  ;[0.15 0 0.007829 0.5] Game Over(Fall Off Tracks)
  (Input|DisableInput 0)
  (Transformation|DetachFromComponent (Variables|Default|GetCamera) "KeepWorld" "KeepWorld" "KeepWorld" false)
  (Variables|Default|SetbGameOver true)
  (Components|Movement|StopMovementImmediately (Variables|Character|GetCharacterMovement))
  (Physics|SetSimulatePhysics (Variables|Default|GetMinecart) true)
  (if (< (Math|Float|Absolute(Float) (.pitch (Variables|/Script/Engine.SceneComponent|GetRelativeRotation (Variables|Default|GetMinecart)))) (Variables|Default|GetManualTiltLimit))
    (Character|LaunchCharacter (+ (Math|Vector|GetForwardVector (Transformation|GetWorldRotation (Variables|Default|GetMinecart))) 1e+05) false false)
    (else
      (Character|LaunchCharacter (* (+ (Math|Vector|RotateVector (Math|Vector|GetForwardVector (Transformation|GetWorldRotation (Variables|Default|GetMinecart))) (Math|Rotator|MakeRotator 0.0 (* _returnvalue_2 9e+01) 0.0)) 1e+06) _returnvalue_2) false false)))
  (Utilities|FlowControl|Delay 2.0)
  (bind _returnvalue_3 (Actor|GetActorOfClass "/Game/Shaon/Minecart/BP_LevelEnd.BP_LevelEnd_C"))
  (Transformation|SetWorldLocation (Variables|Default|GetInteract%20Collision) (Transformation|GetActorLocation _returnvalue_3) false false))

(event Custom|Display%20leaderboard
  ;[0.03632 0.15 0.01788 0.5] Leaderboard
  (UserInterface|Viewport|AddtoViewport (Variables|Score|GetLeaderboard) 0)
  (Utilities|FlowControl|Delay 5.0)
  (Widget|RemovefromParent (Variables|Score|GetLeaderboard)))

(event Custom|ReturnLean
  (bind _minecart (Variables|Default|GetMinecart))
  (bind _relativerotation (Variables|/Script/Engine.SceneComponent|GetRelativeRotation _minecart))
  (bind _pitch (Math|Rotator|BreakRotator _relativerotation))
  ;[0.1894 0.8253 0.8698] Leaning for Minecart
  (if (not (Variables|Default|GetbGameOver))
    (Transformation|AddRelativeRotation _minecart (Math|Rotator|MakeRotator 0.0 (* (Math|Float|SelectFloat -1.0 1.0 (> _pitch 0.0)) (Variables|Default|GetReturnTiltSpeed)) 0.0) false false)
    (if (Math|Float|InRange(Float) _pitch -1.0 1.0)
      (Utilities|Time|ClearandInvalidateTimerbyHandle (Variables|Default|GetReturnLeanTimer)))))

(event Custom|LeftLean
  (bind _minecart (Variables|Default|GetMinecart))
  ;[0.1894 0.8253 0.8698] Leaning for Minecart
  (if (not (<= (.Pitch (Math|Rotator|BreakRotator (Variables|/Script/Engine.SceneComponent|GetRelativeRotation _minecart))) (* (Variables|Default|GetManualTiltLimit) -1.0)))
    (if (not (Variables|Default|GetbGameOver))
      (Transformation|AddRelativeRotation _minecart (Math|Rotator|MakeRotator 0.0 (* (Variables|Default|GetManualTiltRate) -1.0) 0.0) false false))))

(event Custom|NoLean
  ;[0.1894 0.8253 0.8698] Leaning for Minecart
  (if (not (Utilities|Time|IsTimerActivebyHandle (Variables|Default|GetReturnLeanTimer)))
    (if (Variables|Movement|GetbLeaningLeft)
      (Utilities|Time|ClearandInvalidateTimerbyHandle (Variables|Default|GetLeftLeanTimer))
      (Variables|Movement|SetbLeaningLeft false)
      (elif (Variables|Movement|GetbLeaningRight)
        (Utilities|Time|ClearandInvalidateTimerbyHandle (Variables|Default|GetRightLeanTimer))
        (Variables|Movement|SetbLeaningRight false)))
    (bind _returnvalue (Utilities|Time|SetTimerbyEvent (delegate Custom|ReturnLean) 0.01 true))
    (Variables|Default|SetReturnLeanTimer _returnvalue)))

(event Custom|StartLeftLean
  ;[0.1894 0.8253 0.8698] Leaning for Minecart
  (if (not (Variables|Movement|GetbLeaningRight))
    (Utilities|Time|ClearandInvalidateTimerbyHandle (Variables|Default|GetReturnLeanTimer))
    (Utilities|Time|ClearandInvalidateTimerbyHandle (Variables|Default|GetRightLeanTimer))
    (Variables|Movement|SetbLeaningLeft true)
    (bind _returnvalue (Utilities|Time|SetTimerbyEvent (delegate Custom|LeftLean) 0.01 true))
    (Variables|Default|SetLeftLeanTimer _returnvalue)))

(event Custom|SwitchTracks
  ;[0.1905 0.8366 0.8698 0.5] Code to switch the minecart over to another spline
  (if (not (Variables|Movement|GetbIsSwitching))
    (Variables|Movement|SetbIsSwitching true)
    (if (Actor|ActorHasTag (Variables|Movement|GetNextSplineRef) "Broken")
      (bind _output_get (Variables|Movement|SetSplineDistance 0.0 :!label _label))
      (Transformation|SetRelativeTransform (Variables|Collision|GetCapsuleComponent) (Math|Transform|MakeTransform (Math|Vector|MakeVector (.x (.location (Spline|GetTransformatDistanceAlongSpline (Variables|/Game/Orin_Dev/Blueprints/BP_TestingRail_Orin.BP_TestingRail_Orin_C|GetSpline (Variables|Movement|GetNextSplineRef)) _output_get "World" false))) (.y (.location (Spline|GetTransformatDistanceAlongSpline (Variables|/Game/Orin_Dev/Blueprints/BP_TestingRail_Orin.BP_TestingRail_Orin_C|GetSpline (Variables|Movement|GetNextSplineRef)) _output_get "World" false))) (+ (.z (.location (Spline|GetTransformatDistanceAlongSpline (Variables|/Game/Orin_Dev/Blueprints/BP_TestingRail_Orin.BP_TestingRail_Orin_C|GetSpline (Variables|Movement|GetNextSplineRef)) _output_get "World" false))) 1e+02)) (.rotation (Spline|GetTransformatDistanceAlongSpline (Variables|/Game/Orin_Dev/Blueprints/BP_TestingRail_Orin.BP_TestingRail_Orin_C|GetSpline (Variables|Movement|GetNextSplineRef)) _output_get "World" false)) (Variables|/Script/Engine.SceneComponent|GetRelativeScale3D (Variables|Collision|GetCapsuleComponent))) false false)
      (Variables|Movement|SetCurrentSplineRef (Variables|Movement|GetNextSplineRef))
      (Variables|Movement|SetbCanMove true)
      (Utilities|FlowControl|Delay 1.5)
      (Variables|Movement|SetbIsSwitching false)
      (elif (Actor|ActorHasTag (Variables|Movement|GetCurrentSplineRef) "Broken")
        (if (Actor|ActorHasTag (Variables|Movement|GetCurrentSplineRef) "Left")
          (Appearance|SetColorandOpacity (Variables|/Game/Emma_Dev/Widgets/WBP_MinecartMinigame.WBP_MinecartMinigame_C|GetWBP_LeanLeft (Variables|Default|GetMinecarWidget)) (Utilities|Struct|MakeLinearColor 0.0 0.0 0.0 0.0) :!class /Script/UMG.UserWidget)
          (CallFunction|ReceivePoints 50 :!label _label_2)
          (Variables|/Game/Orin_Dev/Blueprints/BP_TestingRail_Orin.BP_TestingRail_Orin_C|SetisActive (Variables|Movement|GetCurrentSplineRef) false :!label _label_3)
          (goto _label)
          (elif (Actor|ActorHasTag (Variables|Movement|GetCurrentSplineRef) "Right")
            (Appearance|SetColorandOpacity (Variables|/Game/Emma_Dev/Widgets/WBP_MinecartMinigame.WBP_MinecartMinigame_C|GetWBP_LeanRight (Variables|Default|GetMinecarWidget)) (Utilities|Struct|MakeLinearColor 0.0 0.0 0.0 0.0) :!class /Script/UMG.UserWidget)
            (goto _label_2)))
        (else
          (goto _label_3))))))

(event Custom|MistimedInput
  (Math|Integer|IncrementInt (Variables|DynamiteThrow|GetMisInputCounter)
    (:%20%20
      (if (>= (Variables|DynamiteThrow|GetMisInputCounter) 2)
        (Variables|DynamiteThrow|SetMisInputCounter 0)
        (Niagara|SpawnSystematLocation "/Game/Violetta_Dev/Particles_VL/VFX/NS_Stylized_Explosion.NS_Stylized_Explosion" (Transformation|GetWorldLocation (Variables|Default|GetPlayerVisual)))
        (CallFunction|EnterStunDelay)))))

(event Custom|SmoothSpeedMultTransitions
  (params (Old%20Speed%20Multiplier :type Float%20%28double-precision%29) (New%20Speed%20Multiplier :type Float%20%28double-precision%29))
  (bind _smoothing (Timeline|Timeline PlayFromStart)
    (:Update
      (Variables|Movement|SetSpeed%20Multiplier (Math|Float|Lerp Old%20Speed%20Multiplier New%20Speed%20Multiplier _smoothing)))))

(event Custom|EnterStunDelay
  (Variables|DynamiteThrow|SetStunned true)
  (Variables|Movement|SetSpeed%20Multiplier (Variables|Movement|GetReverse%20Speed))
  (Utilities|FlowControl|Delay 0.4)
  (CallFunction|SmoothSpeedMultTransitions (Variables|Movement|GetSpeed%20Multiplier) (Variables|Movement|GetStun%20Speed))
  (Utilities|FlowControl|Delay (Variables|DynamiteThrow|GetStunDuration))
  (Variables|DynamiteThrow|SetStunned false)
  (CallFunction|SmoothSpeedMultTransitions (Variables|Movement|GetSpeed%20Multiplier) (Variables|Movement|GetNormal%20Speed)))

(event Custom|StartRightLean
  ;[0.1894 0.8253 0.8698] Leaning for Minecart
  (if (not (Variables|Movement|GetbLeaningLeft))
    (Utilities|Time|ClearandInvalidateTimerbyHandle (Variables|Default|GetReturnLeanTimer))
    (Utilities|Time|ClearandInvalidateTimerbyHandle (Variables|Default|GetLeftLeanTimer))
    (Variables|Movement|SetbLeaningRight true)
    (bind _returnvalue (Utilities|Time|SetTimerbyEvent (delegate Custom|RightLean) 0.01 true))
    (Variables|Default|SetRightLeanTimer _returnvalue)))

(event Custom|TurnSignalLeft
  (bind _minecarwidget (Variables|Default|GetMinecarWidget))
  (bind _wbp_leanleft (Variables|/Game/Emma_Dev/Widgets/WBP_MinecartMinigame.WBP_MinecartMinigame_C|GetWBP_LeanLeft _minecarwidget))
  ;[0.01521 0.06125 0.007499] Makes the Left/Right arrow widget visible when called
  (Appearance|SetColorandOpacity _wbp_leanleft (Utilities|Struct|MakeLinearColor 1.0 0.0 0.0 1.0) :!class /Script/UMG.UserWidget)
  (Utilities|FlowControl|Delay 1.5)
  (Appearance|SetColorandOpacity _wbp_leanleft (Utilities|Struct|MakeLinearColor 0.0 0.0 0.0 0.0) :!class /Script/UMG.UserWidget))

(event Custom|RightLean
  (bind _minecart (Variables|Default|GetMinecart))
  ;[0.1894 0.8253 0.8698] Leaning for Minecart
  (if (not (>= (.Pitch (Math|Rotator|BreakRotator (Variables|/Script/Engine.SceneComponent|GetRelativeRotation _minecart))) (Variables|Default|GetManualTiltLimit)))
    (if (not (Variables|Default|GetbGameOver))
      (Transformation|AddRelativeRotation _minecart (Math|Rotator|MakeRotator 0.0 (Variables|Default|GetManualTiltRate) 0.0) false false))))

(event Custom|TurnSignalRight
  (bind _minecarwidget (Variables|Default|GetMinecarWidget))
  (bind _wbp_leanright (Variables|/Game/Emma_Dev/Widgets/WBP_MinecartMinigame.WBP_MinecartMinigame_C|GetWBP_LeanRight _minecarwidget))
  ;[0.01521 0.06125 0.007499] Makes the Left/Right arrow widget visible when called
  (Appearance|SetColorandOpacity _wbp_leanright (Utilities|Struct|MakeLinearColor 1.0 0.0 0.0 1.0) :!class /Script/UMG.UserWidget)
  (Utilities|FlowControl|Delay 1.5)
  (Appearance|SetColorandOpacity _wbp_leanright (Utilities|Struct|MakeLinearColor 0.0 0.0 0.0 0.0) :!class /Script/UMG.UserWidget))

(event Custom|CustomEvent
  (params (Points :type Integer))
  ;[1 0.9545 0 0.5] Points
  (Variables|Score|SetPoints (+ (Variables|Score|GetPoints) Points)))

(event Input|EnhancedActionEvents|EnhancedInputActionIA_MinecartGo
  (params (ActionValue :type Float%20%28double-precision%29) (ElapsedSeconds :type Float%20%28double-precision%29) (TriggeredSeconds :type Float%20%28double-precision%29) (InputAction :type Input%20Action%20Object%20Reference :default "/Game/Kaitlyn_Dev/IA_MinecartGo.IA_MinecartGo"))
  (bind _minecart (Variables|Default|GetMinecart))
  (bind _bgameover (Variables|Default|GetbGameOver))
  (bind _charactermovement (Variables|Character|GetCharacterMovement))
  (bind _relativerotation (Variables|/Script/Engine.SceneComponent|GetRelativeRotation _minecart))
  ;[0.198 0.8339 0.901] Forward movement with acceleration for minecart
  (:Triggered
    (if (not _bgameover)
      (if (Variables|Movement|GetbCanMove)
        _
        (else
          (Variables|Movement|SetbCanMove true)))
      (Pawn|Input|AddMovementInput (Math|Vector|GetForwardVector (Pawn|GetControlRotation :!class /Script/Engine.Pawn)) ActionValue false)
      (bind _newtrack_0 (Timeline|ForwardRotationTimeline Play)
        (:Update
          (Transformation|SetRelativeRotation (Variables|Default|GetMinecart) (Math|Rotator|MakeRotator _newtrack_0 (.pitch _relativerotation) (.yaw _relativerotation)) false false)
          (bind _output_get (Variables|/Script/Engine.CharacterMovementComponent|SetMaxWalkSpeed _charactermovement (Math|Float|Clamp(Float) (+ (Variables|/Script/Engine.CharacterMovementComponent|GetMaxWalkSpeed _charactermovement) (Variables|Movement|GetSpeedIncrease)) 2e+02 (Variables|Movement|GetMaxSpeed)) :!label _label))
          (Variables|Movement|SetCurrentSpeed _output_get)
          (Utilities|FlowControl|Delay 5.0)
          (goto _label)))))
  (:Completed
    (if (not _bgameover)
      (bind _output_get_2 (Variables|/Script/Engine.CharacterMovementComponent|SetMaxWalkSpeed (Variables|Character|GetCharacterMovement) (Variables|Movement|GetNormalSpeed)))
      (Variables|Movement|SetCurrentSpeed _output_get_2)
      (Timeline|ForwardRotationTimeline Reverse))))

(event Input|EnhancedActionEvents|EnhancedInputActionIA_MinecartBrake
  (params (ActionValue :type Float%20%28double-precision%29) (ElapsedSeconds :type Float%20%28double-precision%29) (TriggeredSeconds :type Float%20%28double-precision%29) (InputAction :type Input%20Action%20Object%20Reference :default "/Game/Kaitlyn_Dev/IA_MinecartBrake.IA_MinecartBrake"))
  (bind _charactermovement (Variables|Character|GetCharacterMovement))
  (bind _minecart (Variables|Default|GetMinecart))
  (bind _bgameover (Variables|Default|GetbGameOver))
  (bind _relativerotation (Variables|/Script/Engine.SceneComponent|GetRelativeRotation _minecart))
  ;[0.1895 0.8301 0.8958] Braking for Minecart
  (:Triggered
    (if (not _bgameover)
      (bind _newtrack_0 (Timeline|BrakeRotationTimeline Play)
        (:Update
          (Transformation|SetRelativeRotation (Variables|Default|GetMinecart) (Math|Rotator|MakeRotator _newtrack_0 (.pitch _relativerotation) (.yaw _relativerotation)) false false)
          (bind _output_get (Variables|/Script/Engine.CharacterMovementComponent|SetMaxWalkSpeed _charactermovement (Math|Float|Clamp(Float) (- (Variables|/Script/Engine.CharacterMovementComponent|GetMaxWalkSpeed _charactermovement) (Variables|Movement|GetBrakingAmount)) 2e+02 (Variables|Movement|GetMaxSpeed)) :!label _label))
          (Variables|Movement|SetCurrentSpeed _output_get)
          (Utilities|FlowControl|Delay 5.0)
          (goto _label)))))
  (:Completed
    (if (not _bgameover)
      (bind _output_get_2 (Variables|/Script/Engine.CharacterMovementComponent|SetMaxWalkSpeed (Variables|Character|GetCharacterMovement) (Variables|Movement|GetNormalSpeed)))
      (Variables|Movement|SetCurrentSpeed _output_get_2)
      (Timeline|BrakeRotationTimeline Reverse))))

(event Input|EnhancedActionEvents|EnhancedInputActionIA_MinecartDuck
  (params (ActionValue :type Boolean) (ElapsedSeconds :type Float%20%28double-precision%29) (TriggeredSeconds :type Float%20%28double-precision%29) (InputAction :type Input%20Action%20Object%20Reference :default "/Game/Kaitlyn_Dev/IA_MinecartDuck.IA_MinecartDuck"))
  (bind _capsulecomponent (Variables|Collision|GetCapsuleComponent))
  (bind _capsulecomponent_2 (Variables|Collision|GetCapsuleComponent))
  (bind _relativelocation (Variables|/Script/Engine.SceneComponent|GetRelativeLocation _capsulecomponent_2))
  (bind _relativelocation_2 (Variables|/Script/Engine.SceneComponent|GetRelativeLocation _capsulecomponent))
  ;[0.1928 0.8446 0.9115] Ducking while in the minecart
  (:Started
    (Transformation|SetRelativeLocation _capsulecomponent (Math|Vector|MakeVector (.x _relativelocation_2) (.y _relativelocation_2) (- (.z _relativelocation_2) 4e+01)) false false))
  (:Completed
    (Transformation|SetRelativeLocation _capsulecomponent_2 (Math|Vector|MakeVector (.x _relativelocation) (.y _relativelocation) (+ (.z _relativelocation) 4e+01)) false false)))

(event Input|EnhancedActionEvents|EnhancedInputActionIA_MinecartLeftLean
  (params (ActionValue :type Boolean) (ElapsedSeconds :type Float%20%28double-precision%29) (TriggeredSeconds :type Float%20%28double-precision%29) (InputAction :type Input%20Action%20Object%20Reference :default "/Game/Kaitlyn_Dev/IA_MinecartLeftLean.IA_MinecartLeftLean"))
  ;[0.1894 0.8253 0.8698] Leaning for Minecart
  (:Started
    (CallFunction|StartLeftLean))
  (:Completed
    (if (not (Variables|Movement|GetbLeaningRight))
      (CallFunction|NoLean))))

(event Input|EnhancedActionEvents|EnhancedInputActionIA_MinecartRightLean
  (params (ActionValue :type Boolean) (ElapsedSeconds :type Float%20%28double-precision%29) (TriggeredSeconds :type Float%20%28double-precision%29) (InputAction :type Input%20Action%20Object%20Reference :default "/Game/Kaitlyn_Dev/IA_MinecartRightLean.IA_MinecartRightLean"))
  ;[0.1894 0.8253 0.8698] Leaning for Minecart
  (:Started
    (CallFunction|StartRightLean))
  (:Completed
    (if (not (Variables|Movement|GetbLeaningLeft))
      (CallFunction|NoLean))))

(event Input|EnhancedActionEvents|EnhancedInputActionIA_Throw
  (params (ActionValue :type Boolean) (ElapsedSeconds :type Float%20%28double-precision%29) (TriggeredSeconds :type Float%20%28double-precision%29) (InputAction :type Input%20Action%20Object%20Reference :default "/Game/Kaitlyn_Dev/IA_Throw.IA_Throw"))
  (bind _ores (Variables|DynamiteThrow|GetOres))
  (bind _minecart (Variables|Default|GetMinecart))
  (bind _dynamiteref (Variables|DynamiteThrow|GetDynamiteRef))
  (bind _dynamiteref_2 (Variables|DynamiteThrow|GetDynamiteRef))
  (bind _dynamiteref_3 (Variables|DynamiteThrow|GetDynamiteRef))
  (bind _returnvalue (Transformation|GetWorldLocation _minecart))
  (bind _output (Utilities|Array|Get(acopy) _dynamiteref_2))
  (bind _output_2 (Utilities|Array|Get(acopy) _dynamiteref_3))
  (bind _output_3 (Utilities|Array|Get(acopy) _dynamiteref))
  (bind (_distance _returnvalue_2) (Actor|FindNearestActor _returnvalue _ores))
  ;[1 0.2599 0.06161 0.5] Throwing for Minecart
  (:Started
    (if (Variables|DynamiteThrow|GetStunned)
      (Development|PrintString "Must wait before throwing agian" true true "(R=0.116767,G=1.000000,B=0.126042,A=1.000000)")
      (elif (Variables|DynamiteThrow|GetbCanThrow)
        (bind _asbp_ores_kaitlyn (Utilities|Casting|CastToBP_Ores_Kaitlyn _returnvalue_2 :!label _label))
        (Utilities|IsValid _asbp_ores_kaitlyn
          (:Is%20Valid
            (bind _output_get (Variables|DynamiteThrow|SetThrowing (< _distance (Variables|DynamiteThrow|GetThrowingRange))))
            (if _output_get
              (Variables|DynamiteThrow|SetMisInputCounter 0)
              (if (not (Variables|/Game/Kaitlyn_Dev/BP_Ores_Kaitlyn.BP_Ores_Kaitlyn_C|GetTargeted _asbp_ores_kaitlyn))
                (Variables|/Game/Kaitlyn_Dev/BP_Ores_Kaitlyn.BP_Ores_Kaitlyn_C|SetTargeted _asbp_ores_kaitlyn true)
                (bind _failed (Default|GetQTEFailState _asbp_ores_kaitlyn))
                (if _failed
                  (Development|PrintString "QTE Failed")
                  (Utilities|Array|RemoveItem (Variables|DynamiteThrow|GetOres) _asbp_ores_kaitlyn)
                  (goto _label)
                  (else
                    (Variables|DynamiteThrow|SetOreLocation (Transformation|GetActorLocation _returnvalue_2))
                    (Utilities|Array|RemoveItem (Variables|DynamiteThrow|GetOres) _asbp_ores_kaitlyn)
                    (Variables|DynamiteThrow|SetbCanThrow false)
                    (Default|StopTimer _asbp_ores_kaitlyn)
                    (bind _returnvalue_3 (Game|SpawnActorfromClass "/Game/Kaitlyn_Dev/BP_Dynamite.BP_Dynamite_C" (Transformation|GetActorTransform) "Undefined" "MultiplyWithRoot" 0 self (Actor|GetComponentbyClass _asbp_ores_kaitlyn "/Script/Engine.SceneComponent") 0))
                    (Utilities|Array|AddUnique (Variables|DynamiteThrow|GetDynamiteRef) _returnvalue_3)
                    (Collision|SetCollisionEnabled (Variables|/Game/Kaitlyn_Dev/BP_Dynamite.BP_Dynamite_C|GetCylinder _returnvalue_3) "NoCollision")
                    (Transformation|AttachComponentToComponent (Utilities|Array|Get(acopy) (Variables|DynamiteThrow|GetDynamiteRef)) (Variables|Default|GetPlayerVisual) "HandGrip_R" "SnapToTarget" "SnapToTarget" "SnapToTarget" true)
                    (bind (_outlaunchvelocity _returnvalue_4) (Game|SuggestProjectileVelocityCustomArc (Transformation|GetWorldLocation (Variables|/Game/Kaitlyn_Dev/BP_Dynamite.BP_Dynamite_C|GetCylinder (Utilities|Array|Get(acopy) (Variables|DynamiteThrow|GetDynamiteRef)))) (Variables|DynamiteThrow|GetOreLocation) 0.0 0.5))
                    (if _returnvalue_4
                      (bind _output_get_2 (Variables|/Script/Engine.MovementComponent|SetVelocity (Variables|/Game/Kaitlyn_Dev/BP_Dynamite.BP_Dynamite_C|GetProjectileMovement _output_2) _outlaunchvelocity))
                      (Variables|/Game/Kaitlyn_Dev/BP_Dynamite.BP_Dynamite_C|SetTargetOre _output_2 (Variables|DynamiteThrow|GetOreLocation))
                      (bind _returnvalue_5 (Class|GameplayStatics|BlueprintPredictProjectilePathAdvanced (Utilities|Struct|MakePredictProjectilePathParams (Transformation|GetWorldLocation (Variables|/Game/Kaitlyn_Dev/BP_Dynamite.BP_Dynamite_C|GetCylinder _output_2)) _output_get_2 true 0.0 5.0 true "ECC_Visibility" "ObjectTypeQuery1")))
                      (if _returnvalue_5
                        (Variables|DynamiteThrow|SetbCanThrow true)
                        (Transformation|DetachFromActor _output_3 "KeepWorld" "KeepWorld" "KeepWorld")
                        (Components|Activation|Activate (Variables|/Game/Kaitlyn_Dev/BP_Dynamite.BP_Dynamite_C|GetProjectileMovement _output_3) false)
                        (Utilities|FlowControl|Delay 0.1)
                        (Collision|SetCollisionEnabled (Variables|/Game/Kaitlyn_Dev/BP_Dynamite.BP_Dynamite_C|GetCylinder (Utilities|Array|Get(acopy) (Variables|DynamiteThrow|GetDynamiteRef))) "QueryAndPhysics")
                        (Physics|SetSimulatePhysics (Variables|/Game/Kaitlyn_Dev/BP_Dynamite.BP_Dynamite_C|GetCylinder (Utilities|Array|Get(acopy) (Variables|DynamiteThrow|GetDynamiteRef))) true)
                        (Class|PrimitiveComponent|AddVelocityChangeImpulseatLocation (Variables|/Game/Kaitlyn_Dev/BP_Dynamite.BP_Dynamite_C|GetCylinder _output) (* (Variables|/Script/Engine.MovementComponent|GetVelocity (Variables|/Game/Kaitlyn_Dev/BP_Dynamite.BP_Dynamite_C|GetProjectileMovement _output)) 1.0) (Transformation|GetWorldLocation (Variables|/Game/Kaitlyn_Dev/BP_Dynamite.BP_Dynamite_C|GetCylinder _output)) "None")
                        (Variables|DynamiteThrow|SetThrowing false)
                        (Default|OreLockon (Utilities|Array|Get(acopy) (Variables|DynamiteThrow|GetDynamiteRef)))
                        (Utilities|FlowControl|Delay 0.5)
                        (Variables|DynamiteThrow|SetbCanThrow true))))))
              (else
                (Development|PrintString "too far")
                (CallFunction|MistimedInput)))))
        (else
          (CallFunction|MistimedInput))))))

(event EventBeginPlay
  ;[0.15 0.15 0.15 0.5] Startup widget creation and variable values being assigned
  (bind _returnvalue (UserInterface|CreateWidget "/Game/Emma_Dev/Widgets/WBP_MinecartMinigame.WBP_MinecartMinigame_C"))
  (Variables|Default|SetMinecarWidget _returnvalue)
  (UserInterface|Viewport|AddtoViewport _returnvalue 0)
  (CallFunction|SetupInputs)
  (bind _outactors (Actor|GetAllActorsOfClasswithTag "/Game/Orin_Dev/Blueprints/BP_TestingRail_Orin.BP_TestingRail_Orin_C" "StartPoint"))
  (Variables|Movement|SetCurrentSplineRef (Utilities|Array|Get(acopy) _outactors))
  (bind _returnvalue_2 (UserInterface|CreateWidget "/Game/Shaon/Widgets/W_Leaderboard.W_Leaderboard_C"))
  (Variables|Score|SetLeaderboard _returnvalue_2)
  (bind _returnvalue_3 (UserInterface|CreateWidget "/Game/Emma_Dev/Widgets/WBP_PauseMenu.WBP_PauseMenu_C"))
  (Variables|Default|SetPauseMenu _returnvalue_3)
  (bind _outactors_2 (Actor|GetAllActorsOfClass "/Game/Kaitlyn_Dev/BP_Ores_Kaitlyn.BP_Ores_Kaitlyn_C"))
  (Variables|DynamiteThrow|SetOres _outactors_2)
  (Variables|Movement|SetbIsSwitching false)
  (Variables|Movement|SetbLeaningRight false)
  (Variables|Movement|SetbLeaningLeft false))

(event Collision|EventActorBeginOverlap
  (params (OtherActor :type Actor%20Object%20Reference)))

(event EventTick
  (params (DeltaSeconds :type Float%20%28single-precision%29))
  (bind _speed_multiplier (Variables|Movement|GetSpeed%20Multiplier))
  (bind _minecart (Variables|Default|GetMinecart))
  (bind _charactermovement (Variables|Character|GetCharacterMovement))
  (bind _returnvalue (Transformation|GetWorldRotation _minecart))
  (bind _maxwalkspeed (Variables|/Script/Engine.CharacterMovementComponent|GetMaxWalkSpeed _charactermovement))
  (bind _returnvalue_2 (/ (.roll _returnvalue) 1.8e+02))
  (bind _returnvalue_3 (* DeltaSeconds _maxwalkspeed))
  (bind _returnvalue_4 (* _returnvalue_2 3.0))
  (bind _returnvalue_5 (+ _speed_multiplier _returnvalue_4))
  (bind _returnvalue_6 (* _returnvalue_3 _returnvalue_5))
  ;[0.08866 0.3864 0.4072] Movement along a spline
  (Development|PrintString (Utilities|String|ToString(Integer) (Variables|Score|GetPoints)) true true "(R=0.000000,G=0.660000,B=1.000000,A=1.000000)" DeltaSeconds)
  (if (not (Variables|Default|GetbGameOver))
    (if (Variables|Movement|GetbCanMove)
      (Development|PrintString (Utilities|String|ToString(Float) _returnvalue_5) true true "(R=1.000000,G=0.769871,B=0.000000,A=1.000000)" DeltaSeconds)
      (Variables|Default|SetSpeed _returnvalue_6)
      (bind _output_get (Variables|Movement|SetSplineDistance (+ _returnvalue_6 (Variables|Movement|GetSplineDistance))))
      (Transformation|SetRelativeTransform (Variables|Collision|GetCapsuleComponent) (Math|Transform|MakeTransform (Math|Vector|MakeVector (.x (.location (Spline|GetTransformatDistanceAlongSpline (Variables|/Game/Orin_Dev/Blueprints/BP_TestingRail_Orin.BP_TestingRail_Orin_C|GetSpline (Variables|Movement|GetCurrentSplineRef)) _output_get "World" false))) (.y (.location (Spline|GetTransformatDistanceAlongSpline (Variables|/Game/Orin_Dev/Blueprints/BP_TestingRail_Orin.BP_TestingRail_Orin_C|GetSpline (Variables|Movement|GetCurrentSplineRef)) _output_get "World" false))) (+ (.z (.location (Spline|GetTransformatDistanceAlongSpline (Variables|/Game/Orin_Dev/Blueprints/BP_TestingRail_Orin.BP_TestingRail_Orin_C|GetSpline (Variables|Movement|GetCurrentSplineRef)) _output_get "World" false))) 1e+02)) (.rotation (Spline|GetTransformatDistanceAlongSpline (Variables|/Game/Orin_Dev/Blueprints/BP_TestingRail_Orin.BP_TestingRail_Orin_C|GetSpline (Variables|Movement|GetCurrentSplineRef)) _output_get "World" false)) (Variables|/Script/Engine.SceneComponent|GetRelativeScale3D (Variables|Collision|GetCapsuleComponent))) false false))))

(event EventPoints
  (params (Points :type Integer))
  (Development|PrintString (Utilities|String|ToString(Integer) Points) true true "(R=0.019092,G=1.000000,B=0.000000,A=1.000000)")
  (Variables|Score|SetPoints (+ Points (Variables|Score|GetPoints))))

(event Input|KeyboardEvents|DebugKeyP
  (params (Key :type Key%20Structure :default "None") (ActionValue :type Input%20Action%20Value%20Structure))
  (bind _returnvalue (Game|GetPlayerController 0))
  (bind _pausemenu (Variables|Default|GetPauseMenu))
  (:Pressed
    (Variables|/Script/Engine.PlayerController|SetbShowMouseCursor _returnvalue true)
    (Input|SetInputModeUIOnly _returnvalue _pausemenu "DoNotLock" false)
    (UserInterface|Viewport|AddtoViewport _pausemenu 0)))

(fn ConstructionScript)

(fn SetupInputs
  (Input|AddMappingContext (PlayerController|LocalPlayerSubsystems|GetEnhancedInputLocalPlayerSubsystem (Game|GetPlayerController 0)) "/Game/Kaitlyn_Dev/IMC_Minecart.IMC_Minecart" 0 "(bIgnoreAllPressedKeysUntilRelease=True,bForceImmediately=False,bNotifyUserSettings=False)"))

(fn GetPoints
  (return 0))

(fn Interact
  (params (Interactor :type Character%20Object%20Reference)))