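; BP_RailwayObstacleL is a railway obstacle that the minecart must lean right to avoid, awarding points as the cart passes.
; Overlapping Box without leaning right stuns the cart and reduces the obstacle's point value once.
; ScoreBox awards the current value once on entry and hides the minecart widget's left warning on exit.
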(event `self.ScoreBox.OnComponentBeginOverlap`
  (params (OverlappedComponent :type "PrimitiveComponent Object Reference") (OtherActor :type "Actor Object Reference") (OtherComp :type "PrimitiveComponent Object Reference") (OtherBodyIndex :type Integer) (bFromSweep :type Boolean) (SweepResult :type "HitResult Structure (by ref)"))
  ;[0.8958 0.84 0.04416 0.5] Adds the Points once passed
  (bind _asbp_minecart_copy_orin (cast `/Game/Orin_Dev/Blueprints/BP_Minecart_Copy_Orin` OtherActor))
  (`/Engine/EditorBlueprintResources/StandardMacros.DoOnce` false
    (:`Completed`
      (`/Game/Developer/BenH/Blueprints/BPI_Points.ReceivePoints` _asbp_minecart_copy_orin (`self.PointValue`)))))

(event `self.ReceiveBeginPlay`
  ;[0.8958 0.84 0.04416 0.5] Adds the Points once passed
  ;;[1 0.7482 0 0.5] Assigns Point Value
  (set `self.PointValue` 25))

(event `self.Box.OnComponentBeginOverlap`
  (params (OverlappedComponent :type "PrimitiveComponent Object Reference") (OtherActor :type "Actor Object Reference") (OtherComp :type "PrimitiveComponent Object Reference") (OtherBodyIndex :type Integer) (bFromSweep :type Boolean) (SweepResult :type "HitResult Structure (by ref)"))
  ;[0.6198 0 0.01147 0.5] Checks if the player is leaning, if not it stuns them and reduces point value
  (bind _asbp_minecart_copy_orin (cast `/Game/Orin_Dev/Blueprints/BP_Minecart_Copy_Orin` OtherActor))
  (if (not (`/Game/Orin_Dev/Blueprints/BP_Minecart_Copy_Orin.bLeaningRight` _asbp_minecart_copy_orin))
    (`/Game/Orin_Dev/Blueprints/BP_Minecart_Copy_Orin.EnterStunDelay` _asbp_minecart_copy_orin)
    (`/Engine/EditorBlueprintResources/StandardMacros.DoOnce` false
      (:`Completed`
        (set `self.PointValue` (- (`self.PointValue`) 15))))))

(event `self.ScoreBox.OnComponentEndOverlap`
  (params (OverlappedComponent :type "PrimitiveComponent Object Reference") (OtherActor :type "Actor Object Reference") (OtherComp :type "PrimitiveComponent Object Reference") (OtherBodyIndex :type Integer))
  (bind _asbp_minecart_copy_orin (cast `/Game/Orin_Dev/Blueprints/BP_Minecart_Copy_Orin` OtherActor))
  (`Widget.SetVisibility` (`/Game/Orin_Dev/Widgets/W_TimerTest.W_LeftWarning` (`/Game/Orin_Dev/Blueprints/BP_Minecart_Copy_Orin.MinecarWidget` _asbp_minecart_copy_orin)) "Hidden"))

(fn `UserConstructionScript`)