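; BP_RailwayObstacleR is a railway obstacle that stuns the minecart unless it is leaning left and awards it points for passing.
; An overlap with Box without the left lean triggers the cart's stun delay and lowers the obstacle's point value, with a DoOnce that resets when the cart leaves.
; ScoreBox hands the remaining points to the cart through a one-shot ReceivePoints call.
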(event `self.ReceiveBeginPlay`
  (set `self.PointValue` 25))

(event `self.Box.OnComponentBeginOverlap`
  (params (OverlappedComponent :type "PrimitiveComponent Object Reference") (OtherActor :type "Actor Object Reference") (OtherComp :type "PrimitiveComponent Object Reference") (OtherBodyIndex :type Integer) (bFromSweep :type Boolean) (SweepResult :type "HitResult Structure (by ref)"))
  (bind _asbp_minecart_copy_orin (cast `/Game/Orin_Dev/Blueprints/BP_Minecart_Copy_Orin` OtherActor))
  (if (not (`/Game/Orin_Dev/Blueprints/BP_Minecart_Copy_Orin.bLeaningLeft` _asbp_minecart_copy_orin))
    (`/Game/Orin_Dev/Blueprints/BP_Minecart_Copy_Orin.EnterStunDelay` _asbp_minecart_copy_orin)
    (`/Engine/EditorBlueprintResources/StandardMacros.DoOnce` false :!label _label
      (:`Completed`
        (set `self.PointValue` (- (`self.PointValue`) 5))
        (`KismetSystemLibrary.PrintString` "-5")))))

(event `self.Box.OnComponentEndOverlap`
  (params (OverlappedComponent :type "PrimitiveComponent Object Reference") (OtherActor :type "Actor Object Reference") (OtherComp :type "PrimitiveComponent Object Reference") (OtherBodyIndex :type Integer))
  (cast `/Game/Orin_Dev/Blueprints/BP_Minecart_Copy_Orin` OtherActor)
  (goto _label :!via `Reset`))

(event `self.ScoreBox.OnComponentBeginOverlap`
  (params (OverlappedComponent :type "PrimitiveComponent Object Reference") (OtherActor :type "Actor Object Reference") (OtherComp :type "PrimitiveComponent Object Reference") (OtherBodyIndex :type Integer) (bFromSweep :type Boolean) (SweepResult :type "HitResult Structure (by ref)"))
  (bind _asbp_minecart_copy_orin (cast `/Game/Orin_Dev/Blueprints/BP_Minecart_Copy_Orin` OtherActor))
  (`/Engine/EditorBlueprintResources/StandardMacros.DoOnce` false
    (:`Completed`
      (`/Game/Developer/BenH/Blueprints/BPI_Points.ReceivePoints` _asbp_minecart_copy_orin (`self.PointValue`)))))

(fn `UserConstructionScript`)