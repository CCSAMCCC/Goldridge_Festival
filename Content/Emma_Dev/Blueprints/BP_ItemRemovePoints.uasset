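; BP_ItemRemovePoints is a pickup that displays a red "-100" point-loss message when the first-person character overlaps it.
; BeginPlay creates a WBP_PointsWon widget and caches its PointsGained text.
; On overlap, it restyles that text, destroys its AHHGSphere component, shows the widget for two seconds, then removes it and destroys itself.
; The graph only handles this feedback and changes no score value.
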(event `self.ReceiveBeginPlay`
  (bind _returnvalue (`|CreateWidget` "/Game/Emma_Dev/Widgets/WBP_PointsWon.WBP_PointsWon_C"))
  (set `self.Points` _returnvalue)
  (set `self.PointsGained` (`/Game/Emma_Dev/Widgets/WBP_PointsWon.PointsGained` (`self.Points`))))

(event `self.ReceiveActorBeginOverlap`
  (params (OtherActor :type "Actor Object Reference"))
  (bind _pointsgained (`self.PointsGained`))
  (cast `/Game/_Developer/Sam/Blueprints/BP_FirstPersonCharacter_Master` OtherActor)
  (`TextBlock.SetText` _pointsgained "-100")
  (`TextBlock.SetColorAndOpacity` _pointsgained (make `SlateColor` (struct :`R` 1.0 :`G` 0.062945 :`B` 0.041667 :`A` 1.0)))
  (`ActorComponent.K2_DestroyComponent` (`self.AHHGSphere`))
  (`UserWidget.AddToViewport` (`self.Points`) 0)
  (`KismetSystemLibrary.Delay` 2.0)
  (`Widget.RemoveFromParent` (`self.Points`))
  (`self.K2_DestroyActor`))

(fn `UserConstructionScript`)