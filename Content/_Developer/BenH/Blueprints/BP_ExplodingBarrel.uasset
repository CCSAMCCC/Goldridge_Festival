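; An exploding barrel actor that blows up when it receives a SendDamage event and damages the actors around it.
; BlastRadius overlap events, seeded on BeginPlay, maintain an array of actors in range, with debug prints on enter and exit.
; Explode spawns a Niagara effect and sound, sends a damage message to each tracked actor, then calls DestroyActor, which sits inside the loop body when the array is not empty.
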(event `self.ReceiveBeginPlay`
  (`KismetArrayLibrary.Array_Append` (`self.ActorsInBlastRadius`) (`PrimitiveComponent.GetOverlappingActors` (`self.BlastRadius`) null)))

(event `self.BlastRadius.OnComponentBeginOverlap`
  (params (OverlappedComponent :type "PrimitiveComponent Object Reference") (OtherActor :type "Actor Object Reference") (OtherComp :type "PrimitiveComponent Object Reference") (OtherBodyIndex :type Integer) (bFromSweep :type Boolean) (SweepResult :type "HitResult Structure (by ref)"))
  (`KismetArrayLibrary.Array_Add` (`self.ActorsInBlastRadius`) OtherActor)
  (`KismetSystemLibrary.PrintString` "In Blast Radius")
  (`KismetSystemLibrary.PrintString` (`KismetSystemLibrary.GetDisplayName` OtherActor)))

(event `self.BlastRadius.OnComponentEndOverlap`
  (params (OverlappedComponent :type "PrimitiveComponent Object Reference") (OtherActor :type "Actor Object Reference") (OtherComp :type "PrimitiveComponent Object Reference") (OtherBodyIndex :type Integer))
  (`KismetArrayLibrary.Array_RemoveItem` (`self.ActorsInBlastRadius`) OtherActor)
  (`KismetSystemLibrary.PrintString` "Outside Blast Redius"))

(event `/Game/_Developer/BenH/Blueprints/Interfaces/BPI_Secondary.Explode`
  (bind _returnvalue (`self.K2_GetActorLocation`))
  (bind _actorsinblastradius (`self.ActorsInBlastRadius`))
  (`NiagaraFunctionLibrary.SpawnSystemAtLocation` "/Game/Violetta_Dev/Particles_VL/VFX/NS_Stylized_Explosion.NS_Stylized_Explosion" _returnvalue (struct) (11.0 11.0 11.0))
  (`GameplayStatics.PlaySoundAtLocation` "/Game/_Developer/BenH/Blueprints/Explosion.Explosion" _returnvalue (struct) 1.0 1.0 0.0 "/Game/_Developer/BenH/Blueprints/ExplosionAttenuation.ExplosionAttenuation" null null null)
  (if (`KismetArrayLibrary.Array_IsEmpty` _actorsinblastradius)
    (`self.K2_DestroyActor`)
    (else
      (for _array_element _actorsinblastradius
        (message `/Game/Shaon/BPI_Damage.SendDamage` _array_element (`self.Damage`))
        (`self.K2_DestroyActor`)))))

(event `/Game/Shaon/BPI_Damage.SendDamage`
  (params (Damage :type Integer))
  (`/Game/_Developer/BenH/Blueprints/Interfaces/BPI_Secondary.Explode`))

(fn `UserConstructionScript`)