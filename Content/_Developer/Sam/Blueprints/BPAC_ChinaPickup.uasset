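; BPAC_ChinaPickup is a developer actor component for picking up china bowls, still mostly stubbed.
; On BeginPlay it casts and caches the first-person player character.
; The overlap event, weight check and pickup function are placeholders, with CheckWeight returning zero.
; Disconnected logic would show a pickup prompt widget when the interactible list is not empty.
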(event `self.ReceiveBeginPlay`
  (bind _asbp_first_person_character_master (cast `/Game/_Developer/Sam/Blueprints/BP_FirstPersonCharacter_Master` (`GameplayStatics.GetPlayerCharacter` 0)))
  (set `self.playercharacter` _asbp_first_person_character_master))

(event `ChinaOverlap`)

(fn `CheckWeight`
  (returns (Weight :type Integer))
  (return 0))

(fn `PickupChina`
  (params (Weight :type Integer) (ChinaBowlActor :type "/Game/_Developer/BenH/Blueprints/BP_ChinaBowl Object Reference"))
  (returns (`WasPickedUp?` :type Boolean)))