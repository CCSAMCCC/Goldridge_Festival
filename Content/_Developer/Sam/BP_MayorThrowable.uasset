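; BP_MayorThrowable is a projectile lobbed by the BP_BOSSAI boss at the player.
; On BeginPlay it makes the boss its owner and sets a suggested arc velocity from the boss's capsule to the player's current position, without homing.
; After a brief arming delay, overlapping anything but the boss triggers an explosion effect and destroys it, as does a fuse of about three seconds.
; No damage is applied here; LockOnPlayer is empty.
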(event `self.ReceiveBeginPlay`
  (bind _returnvalue (`GameplayStatics.GetActorOfClass` "/Game/JP_Dev/Boss/BP_BOSSAI.BP_BOSSAI_C"))
  (bind _output_get (set `self.Boss` _returnvalue))
  (`self.SetOwner` _output_get)
  (`PrimitiveComponent.IgnoreActorWhenMoving` (`self.Box`) (`self.GetOwner`) true)
  (bind _returnvalue_2 (`GameplayStatics.GetActorOfClass` "/Game/JP_Dev/Boss/BP_BOSSAI.BP_BOSSAI_C"))
  (bind _outlaunchvelocity (`GameplayStatics.SuggestProjectileVelocity_CustomArc` (`SceneComponent.K2_GetComponentLocation` (`Character.CapsuleComponent` _returnvalue_2)) (`self.K2_GetActorLocation` (`GameplayStatics.GetPlayerCharacter` 0))))
  (set `MovementComponent.Velocity` _outlaunchvelocity (`self.ProjectileMovement`))
  (set `self.bCanExplode?` false)
  (`KismetSystemLibrary.Delay` 0.2)
  (set `self.bCanExplode?` true)
  (`KismetSystemLibrary.Delay` 2.7)
  (`NiagaraFunctionLibrary.SpawnSystemAtLocation` "/Game/Violetta_Dev/Particles_VL/VFX/NS_Stylized_Explosion.NS_Stylized_Explosion" (`SceneComponent.K2_GetComponentLocation` (`self.Cylinder`)) (struct) (3.0 3.0 3.0))
  (`self.K2_DestroyActor`))

(event `self.Box.OnComponentBeginOverlap`
  (params (OverlappedComponent :type "PrimitiveComponent Object Reference") (OtherActor :type "Actor Object Reference") (OtherComp :type "PrimitiveComponent Object Reference") (OtherBodyIndex :type Integer) (bFromSweep :type Boolean) (SweepResult :type "HitResult Structure (by ref)"))
  (if (`self.bCanExplode?`)
    (if (== OtherActor (`self.Boss`))
      (`KismetSystemLibrary.PrintString` "oops")
      (else
        (`/Engine/EditorBlueprintResources/StandardMacros.DoOnce` false
          (:`Completed`
            (`KismetSystemLibrary.DelayUntilNextFrame`)
            (`KismetSystemLibrary.DelayUntilNextFrame`)
            (`NiagaraFunctionLibrary.SpawnSystemAtLocation` "/Game/Violetta_Dev/Particles_VL/VFX/NS_Stylized_Explosion.NS_Stylized_Explosion" (`SceneComponent.K2_GetComponentLocation` (`self.Cylinder`)) (struct) (3.0 3.0 3.0))
            (`self.K2_DestroyActor`)))))))

(event `LockOnPlayer`)

(fn `UserConstructionScript`)