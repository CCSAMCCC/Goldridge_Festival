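; BP_Dynamite is an explosive actor that bursts in a Niagara effect and destroys itself three seconds after BeginPlay.
; Its cylinder's first overlap with a BP_Ores_Kaitlyn sends that ore's points to the Player, explodes, then calls DynamiteSuccess on the ore.
; OreLockOn removes it from the Player's DynamiteRef, then uses a timeline lerp to zip it to TargetOre before hiding and exploding.
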(event `self.ReceiveBeginPlay`
  (`KismetSystemLibrary.Delay` 3.0)
  (`NiagaraFunctionLibrary.SpawnSystemAtLocation` "/Game/Violetta_Dev/Particles_VL/VFX/NS_Stylized_Explosion.NS_Stylized_Explosion" (`SceneComponent.K2_GetComponentLocation` (`self.Cylinder`)) (struct) (3.0 3.0 3.0))
  (`self.K2_DestroyActor`))

(event `self.Cylinder.OnComponentBeginOverlap`
  (params (OverlappedComponent :type "PrimitiveComponent Object Reference") (OtherActor :type "Actor Object Reference") (OtherComp :type "PrimitiveComponent Object Reference") (OtherBodyIndex :type Integer) (bFromSweep :type Boolean) (SweepResult :type "HitResult Structure (by ref)"))
  (bind _asbp_ores_kaitlyn (cast `/Game/Kaitlyn_Dev/BP_Ores_Kaitlyn` OtherActor))
  (`/Engine/EditorBlueprintResources/StandardMacros.DoOnce` false
    (:`Completed`
      (message `/Game/_Developer/BenH/Blueprints/BPI_Points.ReceivePoints` (`self.Player`) (`/Game/Kaitlyn_Dev/BP_Ores_Kaitlyn.Points` _asbp_ores_kaitlyn))
      (`KismetSystemLibrary.DelayUntilNextFrame`)
      (`KismetSystemLibrary.DelayUntilNextFrame`)
      (`NiagaraFunctionLibrary.SpawnSystemAtLocation` "/Game/Violetta_Dev/Particles_VL/VFX/NS_Stylized_Explosion.NS_Stylized_Explosion" (`SceneComponent.K2_GetComponentLocation` (`self.Cylinder`)) (struct) (3.0 3.0 3.0))
      (`/Engine/EditorBlueprintResources/StandardMacros.IsValid` _asbp_ores_kaitlyn
        (:`Is Valid`
          (`/Game/Kaitlyn_Dev/BP_Ores_Kaitlyn.DynamiteSuccess` _asbp_ores_kaitlyn)
          (`self.K2_DestroyActor`))))))

(event `OreLockOn`
  (`KismetArrayLibrary.Array_RemoveItem` (`/Game/Kaitlyn_Dev/BP_Minecart_Kaitlyn.DynamiteRef` (`self.Player`)) self)
  (`KismetSystemLibrary.Delay` 0.5)
  (set `self.StartPoint` (`SceneComponent.K2_GetComponentLocation` (`self.Cylinder`)))
  (bind (_direction _zip) (`Timeline|Zip to target` :!via `PlayFromStart`)
    (:`Update`
      (`SceneComponent.K2_SetWorldLocation` (`self.DefaultSceneRoot`) (`KismetMathLibrary.VLerp` (`self.StartPoint`) (`self.TargetOre`) (`KismetMathLibrary.FClamp` (* _zip 2.0))) false false)
      (`SceneComponent.K2_SetWorldLocation` (`self.Cylinder`) (`KismetMathLibrary.VLerp` (`self.StartPoint`) (`self.TargetOre`) (`KismetMathLibrary.FClamp` (* _zip 2.0))) false false))
    (:`Finished`
      (`self.SetActorHiddenInGame` true)
      (`KismetSystemLibrary.Delay` 0.2)
      (`NiagaraFunctionLibrary.SpawnSystemAtLocation` "/Game/Violetta_Dev/Particles_VL/VFX/NS_Stylized_Explosion.NS_Stylized_Explosion" (`SceneComponent.K2_GetComponentLocation` (`self.Cylinder`)) (struct) (3.0 3.0 3.0))
      (`self.K2_DestroyActor`))))

(fn `UserConstructionScript`)