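; Player-controlled minecart that rides the level's first BP_SplinePath; interacting loads the minecart test level.
; Once first accelerated, Tick advances it along the spline using MaxWalkSpeed, which go and brake inputs adjust.
; Timelines tilt the cart for acceleration, braking and leaning, with prolonged left lean triggering game over; ducking lowers the capsule.
; Throwing spawns hand-attached dynamite, arcing toward the nearest gold ore found upon overlap.
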(event `self.ReceiveBeginPlay`
  (`self.Setup Inputs`)
  (bind _outactors (`GameplayStatics.GetAllActorsOfClass` "/Game/Kaitlyn_Dev/BP_SplinePath.BP_SplinePath_C"))
  (set `self.SplineRef` (`|GetArrayItem` _outactors)))

(event `self.ReceiveTick`
  (params (DeltaSeconds :type "Float (single-precision)"))
  ; Movement along a spline
  (if (`self.bCanMove`)
    (bind _output_get (set `self.SplineDistance` (+ (* DeltaSeconds (`CharacterMovementComponent.MaxWalkSpeed` (`self.CharacterMovement`))) (`self.SplineDistance`))))
    (bind _returnvalue (`SplineComponent.GetTransformAtDistanceAlongSpline` (`/Game/Kaitlyn_Dev/BP_SplinePath.Spline` (`self.SplineRef`)) _output_get "World" false))
    (`SceneComponent.K2_SetRelativeTransform` (`self.CapsuleComponent`) (`KismetMathLibrary.MakeTransform` (`KismetMathLibrary.MakeVector` (.x (.location _returnvalue)) (.y (.location _returnvalue)) (+ (.z (.location _returnvalue)) 100.0)) (.rotation _returnvalue) (`SceneComponent.RelativeScale3D` (`self.CapsuleComponent`))) false false)))

(event `EnhancedInput|/Game/Kaitlyn_Dev/IA_MinecartGo`
  (params (ActionValue :type "Float (double-precision)") (ElapsedSeconds :type "Float (double-precision)") (TriggeredSeconds :type "Float (double-precision)") (InputAction :type "InputAction Object Reference" :default "/Game/Kaitlyn_Dev/IA_MinecartGo.IA_MinecartGo"))
  (bind _charactermovement (`self.CharacterMovement`))
  ; Forward movement with acceleration for minecart
  (:`Triggered`
    (if (not (`self.bCanMove`))
      (set `self.bCanMove` true))
    (`self.AddMovementInput` (`KismetMathLibrary.GetForwardVector` (`self.GetControlRotation`)) ActionValue)
    (bind (_direction _newtrack_0) (`Timeline|ForwardRotationTimeline` :!label _label)
      (:`Update`
        (`SceneComponent.K2_SetRelativeRotation` (`self.Minecart`) (`KismetMathLibrary.MakeRotator` 0.0 _newtrack_0) false false)
        (set `CharacterMovementComponent.MaxWalkSpeed` (`KismetMathLibrary.FClamp` (+ (`CharacterMovementComponent.MaxWalkSpeed` _charactermovement) (`self.SpeedIncrease`)) 200.0 (`self.MaxSpeed`)) _charactermovement :!label _label_2)
        (`KismetSystemLibrary.Delay` 5.0)
        (goto _label_2))))
  (:`Completed`
    (set `CharacterMovementComponent.MaxWalkSpeed` (`self.NormalSpeed`) (`self.CharacterMovement`))
    (goto _label :!via `Reverse`)))

(event `EnhancedInput|/Game/Kaitlyn_Dev/IA_MinecartBrake`
  (params (ActionValue :type "Float (double-precision)") (ElapsedSeconds :type "Float (double-precision)") (TriggeredSeconds :type "Float (double-precision)") (InputAction :type "InputAction Object Reference" :default "/Game/Kaitlyn_Dev/IA_MinecartBrake.IA_MinecartBrake"))
  (bind _charactermovement (`self.CharacterMovement`))
  ; Braking for Minecart
  (:`Triggered`
    (bind (_direction _newtrack_0) (`Timeline|BrakeRotationTimeline` :!label _label_3)
      (:`Update`
        (`SceneComponent.K2_SetRelativeRotation` (`self.Minecart`) (`KismetMathLibrary.MakeRotator` 0.0 _newtrack_0) false false)
        (set `CharacterMovementComponent.MaxWalkSpeed` (`KismetMathLibrary.FClamp` (- (`CharacterMovementComponent.MaxWalkSpeed` _charactermovement) (`self.BrakingAmount`)) 200.0 (`self.MaxSpeed`)) _charactermovement :!label _label_4)
        (`KismetSystemLibrary.Delay` 5.0)
        (goto _label_4))))
  (:`Completed`
    (set `CharacterMovementComponent.MaxWalkSpeed` (`self.NormalSpeed`) (`self.CharacterMovement`))
    (goto _label_3 :!via `Reverse`)))

(event `EnhancedInput|/Game/Kaitlyn_Dev/IA_MinecartLeftLean`
  (params (ActionValue :type Boolean) (ElapsedSeconds :type "Float (double-precision)") (TriggeredSeconds :type "Float (double-precision)") (InputAction :type "InputAction Object Reference" :default "/Game/Kaitlyn_Dev/IA_MinecartLeftLean.IA_MinecartLeftLean"))
  ; Leaning for Minecart
  (:`Triggered`
    (bind (_direction _newtrack_0) (`Timeline|LeftLeanTimeline` :!label _label_5)
      (:`Update`
        (`SceneComponent.K2_SetRelativeRotation` (`self.Minecart`) (`KismetMathLibrary.MakeRotator` _newtrack_0) false false)
        (if (> TriggeredSeconds 5.0)
          (`self.GameOver`)))))
  (:`Completed`
    (goto _label_5 :!via `Reverse`)))

(event `EnhancedInput|/Game/Kaitlyn_Dev/IA_MinecartRightLean`
  (params (ActionValue :type Boolean) (ElapsedSeconds :type "Float (double-precision)") (TriggeredSeconds :type "Float (double-precision)") (InputAction :type "InputAction Object Reference" :default "/Game/Kaitlyn_Dev/IA_MinecartRightLean.IA_MinecartRightLean"))
  ; Leaning for Minecart
  (:`Triggered`
    (bind (_direction _newtrack_0) (`Timeline|LeanRightTimeline` :!label _label_6)
      (:`Update`
        (`SceneComponent.K2_SetRelativeRotation` (`self.Minecart`) (`KismetMathLibrary.MakeRotator` _newtrack_0) false false)
        (if (> 0.0 5.0)
          (`self.GameOver`)))))
  (:`Completed`
    (goto _label_6 :!via `Reverse`)))

(event `EnhancedInput|/Game/Kaitlyn_Dev/IA_MinecartDuck`
  (params (ActionValue :type Boolean) (ElapsedSeconds :type "Float (double-precision)") (TriggeredSeconds :type "Float (double-precision)") (InputAction :type "InputAction Object Reference" :default "/Game/Kaitlyn_Dev/IA_MinecartDuck.IA_MinecartDuck"))
  (bind _capsulecomponent (`self.CapsuleComponent`))
  (bind _capsulecomponent_2 (`self.CapsuleComponent`))
  (bind (_relativelocation_x _relativelocation_y _relativelocation_z) (`KismetMathLibrary.BreakVector` (`SceneComponent.RelativeLocation` _capsulecomponent_2)))
  (bind (_relativelocation_x_2 _relativelocation_y_2 _relativelocation_z_2) (`KismetMathLibrary.BreakVector` (`SceneComponent.RelativeLocation` _capsulecomponent)))
  ; Ducking while in the minecart
  (:`Started`
    (`SceneComponent.K2_SetRelativeLocation` _capsulecomponent (`KismetMathLibrary.MakeVector` _relativelocation_x_2 _relativelocation_y_2 (- _relativelocation_z_2 40.0)) false false)
    (`KismetSystemLibrary.PrintString` "I'm ducking"))
  (:`Completed`
    (`SceneComponent.K2_SetRelativeLocation` _capsulecomponent_2 (`KismetMathLibrary.MakeVector` _relativelocation_x _relativelocation_y (+ _relativelocation_z 40.0)) false false)
    (`KismetSystemLibrary.PrintString` "Returned to normal")))

(event `Key|G`
  (params (Key :type "Key Structure"))
  ; Exiting the minecart
  (:`Pressed`
    (`KismetSystemLibrary.PrintString` "Exiting minecart")
    (`GameplayStatics.OpenLevelBySoftObjectPtr` "/Game/Kaitlyn_Dev/Lvl_1stPersonTesting.Lvl_1stPersonTesting") ; Change this to level you you want to return to
  ))

(event `GameOver`
  (`self.DisableInput` null)
  (`KismetSystemLibrary.PrintString` "Game Over!"))

(event `EnhancedInput|/Game/Kaitlyn_Dev/IA_Throw`
  (params (ActionValue :type Boolean) (ElapsedSeconds :type "Float (double-precision)") (TriggeredSeconds :type "Float (double-precision)") (InputAction :type "InputAction Object Reference" :default "/Game/Kaitlyn_Dev/IA_Throw.IA_Throw"))
  (bind _dynamiteref (`self.DynamiteRef`))
  (bind _dynamiteref_2 (`self.DynamiteRef`))
  (:`Triggered`
    (`self.K2_DetachFromActor` _dynamiteref_2 "KeepWorld" "KeepWorld" "KeepWorld")
    (`ActorComponent.Activate` (`/Game/Kaitlyn_Dev/BP_Dynamite.ProjectileMovement` _dynamiteref_2) false)
    (`KismetSystemLibrary.Delay` 0.2)
    (`PrimitiveComponent.SetCollisionEnabled` (`/Game/Kaitlyn_Dev/BP_Dynamite.Cylinder` (`self.DynamiteRef`)) "QueryAndPhysics")
    (`PrimitiveComponent.SetSimulatePhysics` (`/Game/Kaitlyn_Dev/BP_Dynamite.Cylinder` (`self.DynamiteRef`)) true)
    (`PrimitiveComponent.AddVelocityChangeImpulseAtLocation` (`/Game/Kaitlyn_Dev/BP_Dynamite.Cylinder` (`self.DynamiteRef`)) (`MovementComponent.Velocity` (`/Game/Kaitlyn_Dev/BP_Dynamite.ProjectileMovement` (`self.DynamiteRef`))) (`SceneComponent.K2_GetComponentLocation` (`/Game/Kaitlyn_Dev/BP_Dynamite.Cylinder` (`self.DynamiteRef`))) "None")
    (`KismetSystemLibrary.Delay` 1.0)
    (`self.K2_DestroyActor` (`self.DynamiteRef`)))
  (:`Started`
    (bind _returnvalue (`|SpawnActorFromClass` "/Game/Kaitlyn_Dev/BP_Dynamite.BP_Dynamite_C" (`self.GetTransform`) "Undefined" "MultiplyWithRoot" null null))
    (set `self.DynamiteRef` _returnvalue)
    (`PrimitiveComponent.SetCollisionEnabled` (`/Game/Kaitlyn_Dev/BP_Dynamite.Cylinder` _returnvalue) "NoCollision")
    (`self.K2_AttachToComponent` (`self.DynamiteRef`) (`self.PlayerVisual`) "HandGrip_R" "SnapToTarget" "SnapToTarget" "SnapToTarget" true)
    (if (`self.bOverlappedGoldOre`)
      (bind _outactors (`GameplayStatics.GetAllActorsOfClass` "/Game/Kaitlyn_Dev/BP_TempGoldOre.BP_TempGoldOre_C"))
      (else
        (`KismetSystemLibrary.PrintString` "No overlapped Gold")))
    (bind (_outlaunchvelocity _returnvalue_2) (`GameplayStatics.SuggestProjectileVelocity_CustomArc` (`SceneComponent.K2_GetComponentLocation` (`/Game/Kaitlyn_Dev/BP_Dynamite.Cylinder` (`self.DynamiteRef`))) (`self.K2_GetActorLocation` (`.ReturnValue` (`GameplayStatics.FindNearestActor` (`SceneComponent.K2_GetComponentLocation` (`self.Minecart`)) _outactors)))))
    (if _returnvalue_2
      (bind _output_get (set `MovementComponent.Velocity` _outlaunchvelocity (`/Game/Kaitlyn_Dev/BP_Dynamite.ProjectileMovement` _dynamiteref)))
      (`GameplayStatics.Blueprint_PredictProjectilePath_Advanced` (make `PredictProjectilePathParams` :`StartLocation` (`SceneComponent.K2_GetComponentLocation` (`/Game/Kaitlyn_Dev/BP_Dynamite.Cylinder` _dynamiteref)) :`LaunchVelocity` _output_get :`bTraceWithCollision` true :`MaxSimTime` 5.0 :`TraceChannel` "ECC_Visibility" :`DrawDebugType` "ForDuration")))))

(event `self.Gold Ore Collision.OnComponentBeginOverlap`
  (params (OverlappedComponent :type "PrimitiveComponent Object Reference") (OtherActor :type "Actor Object Reference") (OtherComp :type "PrimitiveComponent Object Reference") (OtherBodyIndex :type Integer) (bFromSweep :type Boolean) (SweepResult :type "HitResult Structure (by ref)"))
  (cast `/Game/Kaitlyn_Dev/BP_TempGoldOre` OtherActor)
  (set `self.bOverlappedGoldOre` true))

(event `self.Gold Ore Collision.OnComponentEndOverlap`
  (params (OverlappedComponent :type "PrimitiveComponent Object Reference") (OtherActor :type "Actor Object Reference") (OtherComp :type "PrimitiveComponent Object Reference") (OtherBodyIndex :type Integer))
  (set `self.bOverlappedGoldOre` false))

(fn `Interact`
  (params (Interactor :type "Character Object Reference"))
  (returns (Success :type Boolean))
  (`KismetSystemLibrary.PrintString` "Getting into Minecart!")
  (`GameplayStatics.OpenLevelBySoftObjectPtr` "/Game/Kaitlyn_Dev/Lvl_MinecartTests.Lvl_MinecartTests")
  (return false))

(fn `Setup Inputs`
  (`EnhancedInputSubsystemInterface.AddMappingContext` (pcsubsystem `EnhancedInputLocalPlayerSubsystem` (`GameplayStatics.GetPlayerController` 0)) "/Game/Kaitlyn_Dev/IMC_Minecart.IMC_Minecart" 0 (struct)))

(fn `UserConstructionScript`)