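; BP_Ores_Kaitlyn is an ore actor in the minecart game, carrying a quick-time-event widget and exposing its points and QTE fail state.
; When the minecart first enters AutoTargetCollision, the QTE appears and starts.
; Dynamite hitting HitCollision, or DynamiteSuccess, plays the success animation and destroys the ore, while minecart contact stuns the cart, sends a point deduction and destroys it.
; StopTimer pauses the QTE timer, then destroys the ore after a delay.
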(event `self.Auto Target Collision.OnComponentBeginOverlap`
  (params (OverlappedComponent :type "PrimitiveComponent Object Reference") (OtherActor :type "Actor Object Reference") (OtherComp :type "PrimitiveComponent Object Reference") (OtherBodyIndex :type Integer) (bFromSweep :type Boolean) (SweepResult :type "HitResult Structure (by ref)"))
  (bind _qte (`self.QTE`))
  (cast `/Game/Kaitlyn_Dev/BP_Minecart_Kaitlyn` OtherActor)
  (`/Engine/EditorBlueprintResources/StandardMacros.DoOnce` false
    (:`Completed`
      (`SceneComponent.SetVisibility` _qte true false)
      (bind _asw_qte (cast `/Game/Shaon/Minecart/W_QTE` (`WidgetComponent.GetWidget` _qte)))
      (`/Game/Shaon/Minecart/W_QTE.StartQTE` _asw_qte))))

(event `DynamiteSuccess`
  (bind _asw_qte (cast `/Game/Shaon/Minecart/W_QTE` (`WidgetComponent.GetWidget` (`self.QTE`)) :!label _label))
  (`/Game/Shaon/Minecart/W_QTE.PlaySuccessAnimation` _asw_qte)
  (`KismetSystemLibrary.Delay` 0.5)
  (`self.K2_DestroyActor`))

(event `self.Hit Collision.OnComponentBeginOverlap`
  (params (OverlappedComponent :type "PrimitiveComponent Object Reference") (OtherActor :type "Actor Object Reference") (OtherComp :type "PrimitiveComponent Object Reference") (OtherBodyIndex :type Integer) (bFromSweep :type Boolean) (SweepResult :type "HitResult Structure (by ref)"))
  (cast `/Game/Kaitlyn_Dev/BP_Dynamite` OtherActor
    (:`then`
      (goto _label))
    (:`CastFailed`
      (bind _asbp_minecart_kaitlyn (cast `/Game/Kaitlyn_Dev/BP_Minecart_Kaitlyn` OtherActor))
      (`/Engine/EditorBlueprintResources/StandardMacros.DoOnce` false
        (:`Completed`
          (`/Game/Kaitlyn_Dev/BP_Minecart_Kaitlyn.EnterStunDelay` _asbp_minecart_kaitlyn)
          (message `/Game/_Developer/BenH/Blueprints/BPI_Points.ReceivePoints` _asbp_minecart_kaitlyn (`self.PointDeduction`))
          (`self.K2_DestroyActor`))))))

(event `StopTimer`
  (bind _asw_qte (cast `/Game/Shaon/Minecart/W_QTE` (`WidgetComponent.GetWidget` (`self.QTE`))))
  (`KismetSystemLibrary.K2_PauseTimerHandle` (`/Game/Shaon/Minecart/W_QTE.QTETimerHandle` _asw_qte))
  (`KismetSystemLibrary.Delay` 1.5)
  (`self.K2_DestroyActor`))

(fn `Get Points`
  (returns (`Get Points` :type Integer))
  (return (`self.Points`)))

(fn `GetQTEFailState`
  (returns (Failed :type Boolean))
  (bind _asw_qte (cast `/Game/Shaon/Minecart/W_QTE` (`WidgetComponent.GetWidget` (`self.QTE`))))
  (return (`/Game/Shaon/Minecart/W_QTE.Failed` _asw_qte)))

(fn `UserConstructionScript`)