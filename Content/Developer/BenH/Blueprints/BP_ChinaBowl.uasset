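; A china bowl actor that the player can pick up and that shatters when a South Park bull touches it.
; The construction script sets its mesh and weight from a data table row, and physics is optional at start.
; A pickup trigger toggles the player's prompt and interactible list; grabbing passes weight to the player and, if accepted, attaches the bowl to their hold spot.
; Bull overlap spawns Niagara effects and sound, then destroys it.
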(event `/Game/Developer/BenH/Blueprints/Interfaces/BPI_BullMinigame.GrabChina`
  (params (Player :type "/Game/_Developer/Sam/Blueprints/BP_FirstPersonCharacter_Master Object Reference"))
  (bind _chinaholdspot (`/Game/_Developer/Sam/Blueprints/BP_FirstPersonCharacter_Master.ChinaHoldSpot` Player))
  (bind _china (`self.China`))
  ; Grab Custom Event code. Now it's good :)
  (bind _waspickedup_ (message `/Game/Developer/BenH/Blueprints/Interfaces/BPI_BullMinigame.PickupChina` Player (`self.Weight`) self))
  (if _waspickedup_
    (`PrimitiveComponent.SetSimulatePhysics` (`self.China`) false)
    (`SceneComponent.K2_SetWorldLocation` _china (`SceneComponent.K2_GetComponentLocation` _chinaholdspot) false false)
    (`SceneComponent.K2_AttachToComponent` _china _chinaholdspot "None" "KeepWorld" "KeepWorld" "KeepWorld" true)
    (`KismetArrayLibrary.Array_RemoveItem` (`/Game/_Developer/Sam/Blueprints/BP_FirstPersonCharacter_Master.InteractibleList` Player) self)))

(event `self.ReceiveBeginPlay`
  (if (`self.Physics?`)
    (`PrimitiveComponent.SetSimulatePhysics` (`self.China`) true)))

(event `self.PickupTrigger.OnComponentBeginOverlap`
  (params (OverlappedComponent :type "PrimitiveComponent Object Reference") (OtherActor :type "Actor Object Reference") (OtherComp :type "PrimitiveComponent Object Reference") (OtherBodyIndex :type Integer) (bFromSweep :type Boolean) (SweepResult :type "HitResult Structure (by ref)"))
  (bind _asbp_first_person_character_master (cast `/Game/_Developer/Sam/Blueprints/BP_FirstPersonCharacter_Master` OtherActor))
  (`UserWidget.AddToViewport` (`/Game/_Developer/Sam/Blueprints/BP_FirstPersonCharacter_Master.EPickup` _asbp_first_person_character_master) 0)
  (`KismetArrayLibrary.Array_Add` (`/Game/_Developer/Sam/Blueprints/BP_FirstPersonCharacter_Master.InteractibleList` _asbp_first_person_character_master) self)
  (`KismetSystemLibrary.PrintString` "You Can pick me up"))

(event `self.PickupTrigger.OnComponentEndOverlap`
  (params (OverlappedComponent :type "PrimitiveComponent Object Reference") (OtherActor :type "Actor Object Reference") (OtherComp :type "PrimitiveComponent Object Reference") (OtherBodyIndex :type Integer))
  (bind _asbp_first_person_character_master (cast `/Game/_Developer/Sam/Blueprints/BP_FirstPersonCharacter_Master` OtherActor))
  (`Widget.RemoveFromParent` (`/Game/_Developer/Sam/Blueprints/BP_FirstPersonCharacter_Master.EPickup` _asbp_first_person_character_master))
  (`KismetArrayLibrary.Array_RemoveItem` (`/Game/_Developer/Sam/Blueprints/BP_FirstPersonCharacter_Master.InteractibleList` _asbp_first_person_character_master) self)
  (`KismetSystemLibrary.PrintString` "You can no longer pick me up"))

(event `self.BullTrigger.OnComponentBeginOverlap`
  (params (OverlappedComponent :type "PrimitiveComponent Object Reference") (OtherActor :type "Actor Object Reference") (OtherComp :type "PrimitiveComponent Object Reference") (OtherBodyIndex :type Integer) (bFromSweep :type Boolean) (SweepResult :type "HitResult Structure (by ref)"))
  (bind _returnvalue (`SceneComponent.K2_GetComponentLocation` (`self.China`)))
  (cast `/Game/JP_Dev/Migration/scene/StaticMeshes/BP_SouthParkBull` OtherActor)
  ; Niagra and Destruction Code
  (`NiagaraFunctionLibrary.SpawnSystemAtLocation` "/Game/Developer/BenH/Niagara/NS_ChinaBowl.NS_ChinaBowl" _returnvalue)
  (`GameplayStatics.PlaySoundAtLocation` "/Game/Developer/BenH/Sounds/dragon-studio-glass-breaking-504033.dragon-studio-glass-breaking-504033" _returnvalue (struct) 1.0 1.0 0.0 "/Game/Developer/BenH/Blueprints/ChinaSoundAttenuation.ChinaSoundAttenuation" null null null)
  (`self.K2_DestroyActor`))

(fn `CheckWeight`
  (returns (Weight :type Integer))
  (return (`self.Weight`)))

(fn `PickupChina`
  (params (Weight :type Integer) (ChinaBowlActor :type "/Game/Developer/BenH/Blueprints/BP_ChinaBowl Object Reference"))
  (returns (`WasPickedUp?` :type Boolean))
  (return false))

(fn `UserConstructionScript`
  (bind (_datatable _rowname) (break `DataTableRowHandle` (`self.Selection`)))
  (bind _returnvalue (`|GetDataTableRow` _datatable _rowname)
    (:`then`
      (bind (_mesh _points _weight) (break `/Game/Developer/BenH/DataTables/STRUCT_China` _returnvalue))
      (`StaticMeshComponent.SetStaticMesh` (`self.China`) _mesh)
      (set `self.Weight` _weight))))