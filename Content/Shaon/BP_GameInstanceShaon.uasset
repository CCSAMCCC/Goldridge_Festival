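; Game instance that owns the save game, loading it at startup or creating a new object if none exists.
; Load and save support sync or async slot access, with only async load completion calling OnGameLoaded.
; Bull, Minecart and Shooting minigame data are stored per enum value and written to the slot immediately.
; Aim and ammo upgrade flags update the in-memory save without writing it to disk.
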(event `self.ReceiveInit`
  (`/Game/Shaon/BPI_SaveGame.LoadGameData` false))

(event `/Game/Shaon/BPI_SaveGame.LoadGameData`
  (params (Async :type Boolean))
  (bind _returnvalue (`GameplayStatics.DoesSaveGameExist` (`self.SlotName`)))
  (if _returnvalue
    (if Async
      (bind _savegame (`AsyncActionHandleSaveGame.AsyncLoadGameFromSlot` (`self.SlotName`))
        (:`Completed`
          (bind _asbp_save_game (cast `/Game/Shaon/BP_SaveGame` _savegame))
          (set `self.SavedData` _asbp_save_game)
          (`self.OnGameLoaded`)))
      (else
        (bind _returnvalue_2 (`GameplayStatics.LoadGameFromSlot` (`self.SlotName`)))
        (bind _asbp_save_game_2 (cast `/Game/Shaon/BP_SaveGame` _returnvalue_2))
        (set `self.SavedData` _asbp_save_game_2)))
    (else
      (`KismetSystemLibrary.PrintString` "game data created")
      (bind _returnvalue_3 (`GameplayStatics.CreateSaveGameObject` "/Game/Shaon/BP_SaveGame.BP_SaveGame_C"))
      (set `self.SavedData` _returnvalue_3))))

(event `/Game/Shaon/BPI_SaveGame.SaveGameData`
  (params (Async :type Boolean))
  (if Async
    (`AsyncActionHandleSaveGame.AsyncSaveGameToSlot` (`self.SavedData`) (`self.SlotName`))
    (else
      (`GameplayStatics.SaveGameToSlot` (`self.SavedData`) (`self.SlotName`)))))

(event `/Game/Shaon/BPI_SaveGame.SaveMinigameData`
  (params (MiniGameSave :type "/Game/Shaon/S_Minigame Structure") (Async :type Boolean) (Minigame :type "/Game/Shaon/E_Minigames Enum" :default "NewEnumerator3"))
  (bind _saveddata (`self.SavedData`))
  (switch `/Game/Shaon/E_Minigames` Minigame
    (:`NewEnumerator0`
      (set `/Game/Shaon/BP_SaveGame.BullMiniGameSave` MiniGameSave _saveddata))
    (:`NewEnumerator1`
      (set `/Game/Shaon/BP_SaveGame.MinecartMiniGameSave` MiniGameSave _saveddata))
    (:`NewEnumerator2`
      (set `/Game/Shaon/BP_SaveGame.ShootingMiniGameSave` MiniGameSave _saveddata)))
  (`/Game/Shaon/BPI_SaveGame.SaveGameData` Async))

(event `/Game/Shaon/BPI_SaveGame.SavePlayerUpgrade`
  (params (Upgrade :type "/Game/Shaon/E_Upgrades Enum" :default "NewEnumerator2") (Async :type Boolean))
  (switch `/Game/Shaon/E_Upgrades` Upgrade
    (:`NewEnumerator0`
      (set `self.Upgrades Save Aim Upgrade` true))
    (:`NewEnumerator1`
      (set `self.Upgrades Save Ammo Upgrade` true)))
  (set `/Game/Shaon/BP_SaveGame.UpgradesSave` (make `/Game/Shaon/S_Upgrades` (`self.Upgrades Save Aim Upgrade`) (`self.Upgrades Save Ammo Upgrade`)) (`self.SavedData`)))

(fn `GetGameData`
  (returns (GameData :type "/Game/Shaon/BP_SaveGame Object Reference"))
  (return (`self.SavedData`)))

(fn `GetMinigameData`
  (params (Minigame :type "/Game/Shaon/E_Minigames Enum" :default "NewEnumerator3") (GameData :type "/Game/Shaon/BP_SaveGame Object Reference"))
  (returns (MinigameData :type "/Game/Shaon/S_Minigame Structure"))
  (switch `/Game/Shaon/E_Minigames` Minigame
    (:`NewEnumerator0`
      (return (`/Game/Shaon/BP_SaveGame.BullMiniGameSave` GameData)))
    (:`NewEnumerator1`
      (return (`/Game/Shaon/BP_SaveGame.MinecartMiniGameSave` GameData)))
    (:`NewEnumerator2`
      (return (`/Game/Shaon/BP_SaveGame.ShootingMiniGameSave` GameData)))))