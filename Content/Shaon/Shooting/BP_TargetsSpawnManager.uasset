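; Manager for a shooting minigame that spawns targets and detects when all of them have been destroyed.
; SpawnTargets places a BP_MasterTarget at every BP_TargetSpawner in the level and tracks them in SpawnedTargets.
; TargetDestroyed removes the destroyed target, prints the remaining count, and calls FinishMingameMessage on the player character once none remain.
; BeginPlay only runs a target lookup whose result is unused.
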(event `self.ReceiveBeginPlay`
  (`GameplayStatics.GetAllActorsOfClass` "/Game/_Developer/BenH/Blueprints/BP_MasterTarget.BP_MasterTarget_C"))

(event `SpawnTargets`
  (bind _outactors (`GameplayStatics.GetAllActorsOfClass` "/Game/Shaon/Shooting/BP_TargetSpawner.BP_TargetSpawner_C"))
  (for _array_element _outactors
    (`|SpawnActorFromClass` "/Game/_Developer/BenH/Blueprints/BP_MasterTarget.BP_MasterTarget_C" (`SceneComponent.K2_GetComponentToWorld` (`/Game/Shaon/Shooting/BP_TargetSpawner.DefaultSceneRoot` _array_element)) "AlwaysSpawn" "MultiplyWithRoot" null 0.0 0.0 true false 0.0 null false "/Game/_Developer/BenH/Materials/M_Outline.M_Outline" false null null null 50.0 20.0 100 null)
    (`KismetSystemLibrary.PrintString` "spawned")
    (`KismetArrayLibrary.Array_AddUnique` (`self.SpawnedTargets`))))

(event `TargetDestroyed`
  (params (DestroyedChina :type "/Game/Shaon/Bull/BP_ChinaBowlShaon2 Object Reference (by ref)"))
  (bind _spawnedtargets (`self.SpawnedTargets`))
  (`KismetArrayLibrary.Array_RemoveItem` _spawnedtargets DestroyedChina)
  (if (`KismetArrayLibrary.Array_IsEmpty` _spawnedtargets)
    (`KismetSystemLibrary.PrintString` "no targets remaining")
    (message `/Game/Shaon/BPI_Minigame.FinishMingame` (`GameplayStatics.GetPlayerCharacter` 0))
    (else
      (`KismetSystemLibrary.PrintText` (`|FormatText` "Targets remaining: {target}" (`KismetArrayLibrary.Array_Length` _spawnedtargets))))))

(fn `UserConstructionScript`)