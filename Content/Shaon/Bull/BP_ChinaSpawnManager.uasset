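; BP_ChinaSpawnManager spawns breakable china bowls for a minigame and detects when all of them are destroyed.
; SpawnChina creates a BP_ChinaBowl at every BP_ChinaSpawner, passing the spawner's Selection and itself as Manager, and tracks each bowl in SpawnedChina.
; ChinaDestroyed removes a bowl from that array, prints the remaining count, and calls FinishMingameMessage on the player character when none remain.
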(event `SpawnChina`
  (bind _outactors (`GameplayStatics.GetAllActorsOfClass` "/Game/Shaon/Bull/BP_ChinaSpawner.BP_ChinaSpawner_C"))
  (for _array_element _outactors
    (bind _returnvalue (`|SpawnActorFromClass` "/Game/_Developer/BenH/Blueprints/BP_ChinaBowl.BP_ChinaBowl_C" (`SceneComponent.K2_GetComponentToWorld` (`/Game/Shaon/Bull/BP_ChinaSpawner.DefaultSceneRoot` _array_element)) "AlwaysSpawn" "MultiplyWithRoot" null (`/Game/Shaon/Bull/BP_ChinaSpawner.Selection` _array_element) false self null))
    (`KismetSystemLibrary.PrintString` "spawned")
    (`KismetArrayLibrary.Array_AddUnique` (`self.SpawnedChina`) _returnvalue)))

(event `ChinaDestroyed`
  (params (DestroyedChina :type "/Game/_Developer/BenH/Blueprints/BP_ChinaBowl Object Reference (by ref)"))
  (bind _spawnedchina (`self.SpawnedChina`))
  (`KismetArrayLibrary.Array_RemoveItem` _spawnedchina DestroyedChina)
  (if (`KismetArrayLibrary.Array_IsEmpty` _spawnedchina)
    (`KismetSystemLibrary.PrintString` "no china remaining")
    (message `/Game/Shaon/BPI_Minigame.FinishMingame` (`GameplayStatics.GetPlayerCharacter` 0))
    (else
      (`KismetSystemLibrary.PrintText` (`|FormatText` "China remaining: {china}" (`KismetArrayLibrary.Array_Length` _spawnedchina))))))

(fn `UserConstructionScript`)