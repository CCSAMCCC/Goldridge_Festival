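; Breakable china bowl prop that simulates physics and reacts when a South Park bull or first-person character overlaps its BullTrigger.
; The construction script sets mesh and weight from the selected data table row, and CheckWeight exposes that weight.
; Either overlap spawns the NS_ChinaBowl Niagara effect and calls play-sound at the bowl.
; Manager notification, actor destruction and score text are unwired, and PickupChina only returns false.
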(event `self.ReceiveBeginPlay`
  (`PrimitiveComponent.SetSimulatePhysics` (`self.China`) true))

(event `self.BullTrigger.OnComponentBeginOverlap`
  (params (OverlappedComponent :type "PrimitiveComponent Object Reference") (OtherActor :type "Actor Object Reference") (OtherComp :type "PrimitiveComponent Object Reference") (OtherBodyIndex :type Integer) (bFromSweep :type Boolean) (SweepResult :type "HitResult Structure (by ref)"))
  (bind _returnvalue (`SceneComponent.K2_GetComponentLocation` (`self.China`)))
  (`|ExecutionSequence`
    (:`then_0`
      (cast `/Game/JP_Dev/Migration/scene/StaticMeshes/BP_SouthParkBull` OtherActor))
    (:`then_1`
      (cast `/Game/_Developer/Sam/Blueprints/BP_FirstPersonCharacter_Master` OtherActor)))
  ; Niagra and Destruction Code
  (`NiagaraFunctionLibrary.SpawnSystemAtLocation` "/Game/_Developer/BenH/Niagara/NS_ChinaBowl.NS_ChinaBowl" _returnvalue)
  (`GameplayStatics.PlaySoundAtLocation` null _returnvalue (struct) 1.0 1.0 0.0 null null null null))

(fn `CheckWeight`
  (returns (Weight :type Integer))
  (return (`self.Weight`)))

(fn `PickupChina`
  (params (Weight :type Integer) (ChinaBowlActor :type "/Game/_Developer/BenH/Blueprints/BP_ChinaBowl Object Reference"))
  (returns (`WasPickedUp?` :type Boolean))
  (return false))

(fn `UserConstructionScript`
  (bind (_datatable _rowname) (break `DataTableRowHandle` (`self.Selection`)))
  (bind _returnvalue (`|GetDataTableRow` _datatable _rowname)
    (:`then`
      (bind (_mesh _points _weight) (break `/Game/_Developer/BenH/DataTables/STRUCT_China` _returnvalue))
      (`StaticMeshComponent.SetStaticMesh` (`self.China`) _mesh)
      (set `self.Weight` _weight))))